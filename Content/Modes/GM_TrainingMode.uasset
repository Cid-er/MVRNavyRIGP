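; Training game mode that coordinates player-driven vessel rotation and switching between the training UI and test menu.
; On BeginPlay it finds the periscope, character and training ship, then binds their events and the menu navigation.
; A character-triggered toggle swaps Enhanced Input mapping contexts between player and vessel, while pitch, yaw and roll events rotate the ship's root locally.
; Exiting the periscope creates and shows a new training widget.
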(event Custom|ExitPeriscope_Event
  (bind _returnvalue (UserInterface|CreateWidget "/Game/UI/TrainingUI.TrainingUI_C"))
  (bind _output_get (Variables|Default|SetTrainingUIWidget _returnvalue))
  (UserInterface|Viewport|AddtoViewport _output_get 0)
  (Development|PrintString "nahhhhhh"))

(event Custom|TriggerVesselControl_Event
  (if (Variables|Default|GetIsPossesingVessel)
    (Variables|Default|SetIsPossesingVessel false)
    (else
      (Variables|Default|SetIsPossesingVessel true)))
  (CallFunction|ChangeIMC)
  (Default|SetControllingText (Variables|Default|GetTrainingUIWidget) (Variables|Default|GetIsPossesingVessel)))

(event Custom|AddPitch
  (params (Pitch :type Float%20%28double-precision%29))
  (Transformation|AddLocalRotation (Variables|/Game/Actors/TrainingMode/BP_TrainingModeShip.BP_TrainingModeShip_C|GetDefaultSceneRoot (Variables|Default|GetTrainingModeVesselRef)) (Math|Rotator|MakeRotator 0.0 Pitch 0.0) false false)
  (Development|PrintString (Utilities|String|ToString(Float) Pitch)))

(event Custom|AddYaw
  (params (Yaw :type Float%20%28double-precision%29))
  (Transformation|AddLocalRotation (Variables|/Game/Actors/TrainingMode/BP_TrainingModeShip.BP_TrainingModeShip_C|GetDefaultSceneRoot (Variables|Default|GetTrainingModeVesselRef)) (Math|Rotator|MakeRotator 0.0 0.0 Yaw) false false)
  (Development|PrintString (Utilities|String|ToString(Float) Yaw)))

(event Custom|AddRoll
  (params (Roll :type Float%20%28double-precision%29))
  (Transformation|AddLocalRotation (Variables|/Game/Actors/TrainingMode/BP_TrainingModeShip.BP_TrainingModeShip_C|GetDefaultSceneRoot (Variables|Default|GetTrainingModeVesselRef)) (Math|Rotator|MakeRotator Roll 0.0 0.0) false false)
  (Development|PrintString (Utilities|String|ToString(Float) Roll)))

(event Custom|GoToTestMenu
  (CallFunction|SetTrainingTestWidget))

(event Custom|BackToTrainingUI
  (CallFunction|SetTrainingUIWidget))

(event EventBeginPlay
  (CallFunction|SetTrainingUIWidget)
  (bind _returnvalue (Actor|GetActorOfClass "/Game/Actors/BP_Periscope.BP_Periscope_C"))
  (bind _output_get (Variables|Default|SetPeriscopeRef _returnvalue))
  (EventDispatchers|AssignExitPeriscope _output_get (delegate Custom|ExitPeriscope_Event))
  (bind _returnvalue_2 (Actor|GetActorOfClass "/Game/FirstPerson/Blueprints/BP_FirstPersonCharacter.BP_FirstPersonCharacter_C"))
  (bind _output_get_2 (Variables|Default|SetCharacterRef _returnvalue_2))
  (EventDispatchers|BindEventtoTriggerVesselControl _output_get_2 (delegate Custom|TriggerVesselControl_Event))
  (EventDispatchers|BindEventtoVesselPitch _output_get_2 (delegate Custom|AddPitch))
  (EventDispatchers|BindEventtoVesselYaw _output_get_2 (delegate Custom|AddYaw))
  (EventDispatchers|BindEventtoVesselRoll _output_get_2 (delegate Custom|AddRoll))
  (bind _returnvalue_3 (Actor|GetActorOfClass "/Game/Actors/TrainingMode/BP_TrainingModeShip.BP_TrainingModeShip_C"))
  (Variables|Default|SetTrainingModeVesselRef _returnvalue_3)
  (EventDispatchers|BindEventtoGotoTrainingTestMenu (Variables|Default|GetTrainingUIWidget) (delegate Custom|GoToTestMenu))
  (EventDispatchers|BindEventtoBacktoTrainingUI (Variables|Default|GetTrainingTestMenu) (delegate Custom|BackToTrainingUI)))

(fn ConstructionScript)

(fn ChangeIMC
  (bind _asplayer_controller (Utilities|Casting|CastToPlayerController (Pawn|GetController (Variables|Default|GetCharacterRef)))
    (:then
      (if (Variables|Default|GetIsPossesingVessel)
        (Input|RemoveMappingContext (PlayerController|LocalPlayerSubsystems|GetEnhancedInputLocalPlayerSubsystem _asplayer_controller) "/Game/Input/IMC_Default.IMC_Default" "(bIgnoreAllPressedKeysUntilRelease=True,bForceImmediately=False,bNotifyUserSettings=False)")
        (Input|AddMappingContext (PlayerController|LocalPlayerSubsystems|GetEnhancedInputLocalPlayerSubsystem _asplayer_controller) "/Game/Input/TrainingMode/IMC_Training.IMC_Training" 0 "(bIgnoreAllPressedKeysUntilRelease=True,bForceImmediately=False,bNotifyUserSettings=False)")
        (Development|PrintString "Controlling vessel")
        (else
          (Input|RemoveMappingContext (PlayerController|LocalPlayerSubsystems|GetEnhancedInputLocalPlayerSubsystem _asplayer_controller) "/Game/Input/TrainingMode/IMC_Training.IMC_Training" "(bIgnoreAllPressedKeysUntilRelease=True,bForceImmediately=False,bNotifyUserSettings=False)")
          (Input|AddMappingContext (PlayerController|LocalPlayerSubsystems|GetEnhancedInputLocalPlayerSubsystem _asplayer_controller) "/Game/Input/IMC_Default.IMC_Default" 0 "(bIgnoreAllPressedKeysUntilRelease=True,bForceImmediately=False,bNotifyUserSettings=False)")
          (Development|PrintString "Controlling player"))))
    (:CastFailed
      (Development|PrintString "Cast to controller failed"))))

(fn SetTrainingUIWidget
  (Viewport|RemoveAllWidgets)
  (UserInterface|Viewport|AddtoViewport (Variables|Default|GetTrainingUIWidget) 0))

(fn SetTrainingTestWidget
  (Viewport|RemoveAllWidgets)
  (UserInterface|Viewport|AddtoViewport (Variables|Default|GetTrainingTestMenu) 0))

(fn GetTrainingTestWidget
  (return (Variables|Default|GetTrainingTestMenu)))