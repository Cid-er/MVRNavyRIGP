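; Game mode for freeplay, where player input rotates a BP_FreemodeVessel while the player character's movement is disabled.
; BeginPlay finds the vessel and character, shows UIWidget with the mouse cursor in game-and-UI input, and adds the IMC_Freemode mapping context, which EndPlay removes.
; It binds to the character's pitch, yaw and roll events, applying each value as local rotation on the vessel's root and printing it.
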(event Custom|Pitch
  (params (Pitch :type Float%20%28double-precision%29))
  (Transformation|AddLocalRotation (Variables|/Script/Engine.Actor|GetRootComponent (Variables|Default|GetFreemodeVesselRef)) (Math|Rotator|MakeRotator 0.0 Pitch 0.0) false false)
  (Development|PrintString (Utilities|String|ToString(Float) Pitch)))

(event Custom|Yaw
  (params (Yaw :type Float%20%28double-precision%29))
  (Transformation|AddLocalRotation (Variables|/Script/Engine.Actor|GetRootComponent (Variables|Default|GetFreemodeVesselRef)) (Math|Rotator|MakeRotator 0.0 0.0 Yaw) false false)
  (Development|PrintString (Utilities|String|ToString(Float) Yaw)))

(event Custom|Roll
  (params (Roll :type Float%20%28double-precision%29))
  (Transformation|AddLocalRotation (Variables|/Script/Engine.Actor|GetRootComponent (Variables|Default|GetFreemodeVesselRef)) (Math|Rotator|MakeRotator Roll 0.0 0.0) false false)
  (Development|PrintString (Utilities|String|ToString(Float) Roll)))

(event EventBeginPlay
  (bind _returnvalue (Game|GetPlayerController 0))
  (bind _uiwidget (Variables|Default|GetUIWidget))
  (bind _returnvalue_2 (Actor|GetActorOfClass "/Game/Actors/Freemode/BP_FreemodeVessel.BP_FreemodeVessel_C"))
  (Variables|Default|SetFreemodeVesselRef _returnvalue_2)
  (bind _returnvalue_3 (Actor|GetActorOfClass "/Game/FirstPerson/Blueprints/BP_FreeplayCharacter.BP_FreeplayCharacter_C"))
  (bind _output_get (Variables|Default|SetPlayerRef _returnvalue_3))
  (Pawn|Components|CharacterMovement|DisableMovement (Variables|/Script/Engine.Character|GetCharacterMovement _output_get))
  (UserInterface|Viewport|AddtoViewport _uiwidget 0)
  (Variables|/Script/Engine.PlayerController|SetbShowMouseCursor _returnvalue true)
  (Input|SetInputModeGameandUI _returnvalue _uiwidget "DoNotLock" false false)
  (CallFunction|SetFreemodeIMC)
  (EventDispatchers|BindEventtoVesselPitch (Variables|Default|GetPlayerRef) (delegate Custom|Pitch))
  (EventDispatchers|BindEventtoVesselYaw (Variables|Default|GetPlayerRef) (delegate Custom|Yaw))
  (EventDispatchers|BindEventtoVesselRoll (Variables|Default|GetPlayerRef) (delegate Custom|Roll)))

(event EventEndPlay
  (params (EndPlayReason :type EEndPlayReason%20Enum :default "Destroyed"))
  (CallFunction|RemoveFreemodeIMC))

(fn ConstructionScript)

(fn SetFreemodeIMC
  (bind _asplayer_controller (Utilities|Casting|CastToPlayerController (Pawn|GetController (Variables|Default|GetPlayerRef))))
  (Input|AddMappingContext (PlayerController|LocalPlayerSubsystems|GetEnhancedInputLocalPlayerSubsystem _asplayer_controller) "/Game/Input/TrainingMode/IMC_Freemode.IMC_Freemode" 0 "(bIgnoreAllPressedKeysUntilRelease=True,bForceImmediately=False,bNotifyUserSettings=False)"))

(fn RemoveFreemodeIMC
  (bind _asplayer_controller (Utilities|Casting|CastToPlayerController (Pawn|GetController (Variables|Default|GetPlayerRef))))
  (Input|RemoveMappingContext (PlayerController|LocalPlayerSubsystems|GetEnhancedInputLocalPlayerSubsystem _asplayer_controller) "/Game/Input/TrainingMode/IMC_Freemode.IMC_Freemode" "(bIgnoreAllPressedKeysUntilRelease=True,bForceImmediately=False,bNotifyUserSettings=False)"))