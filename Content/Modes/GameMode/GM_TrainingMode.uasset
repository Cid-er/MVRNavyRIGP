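; GM_TrainingMode is the game mode for a training mode where the player configures conditions, then runs a vessel test.
; At BeginPlay it freezes character movement, caches the HUD and spawner, ensures a display ship exists and binds the HUD's start and end test dispatchers.
; Starting a test swaps the display ship for a spawned vessel of the chosen threat type and restores walking.
; Ending destroys that vessel, respawns the display ship and freezes movement again.
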(event Custom|StartTest
  (bind _trainingmenuvesselref (Variables|Default|GetTrainingMenuVesselRef))
  ;[0.15 0.15 0.15 0.5] Binding functionality to HUD_TrainingMode Event Dispatchers: Start Test, End Test
  (Variables|Default|SetInTest true)
  (Utilities|IsValid _trainingmenuvesselref
    (:Is%20Valid
      (Actor|DestroyActor _trainingmenuvesselref))
    (:Is%20Not%20Valid
      _))
  (bind _trainingmenuref (Default|GetTrainingMenu (Variables|Default|GetHUDRef)))
  (bind _threattype (Default|GetThreatTypetoSpawn _trainingmenuref))
  (bind _threatactor (Default|SpawnTestVessel (Variables|Default|GetTestSpawnerRef) _threattype))
  (Variables|Default|SetTestVesselRef _threatactor)
  (bind _returnvalue (Actor|GetActorOfClass "/Game/FirstPerson/Blueprints/BP_FirstPersonCharacter.BP_FirstPersonCharacter_C"))
  (Pawn|Components|CharacterMovement|SetMovementMode (Variables|/Script/Engine.Character|GetCharacterMovement _returnvalue) "MOVE_Walking" 0))

(event Custom|EndEvent
  (bind _testvesselref (Variables|Default|GetTestVesselRef))
  ;[0.15 0.15 0.15 0.5] Binding functionality to HUD_TrainingMode Event Dispatchers: Start Test, End Test
  (Variables|Default|SetInTest false)
  (Utilities|IsValid _testvesselref
    (:Is%20Valid
      (Actor|DestroyActor _testvesselref))
    (:Is%20Not%20Valid
      _))
  (CallFunction|SpawnDisplayVessel)
  (bind _returnvalue (Actor|GetActorOfClass "/Game/FirstPerson/Blueprints/BP_FirstPersonCharacter.BP_FirstPersonCharacter_C"))
  (Pawn|Components|CharacterMovement|DisableMovement (Variables|/Script/Engine.Character|GetCharacterMovement _returnvalue)))

(event EventBeginPlay
  ;[0.15 0.15 0.15 0.5] Disables Character Movement while player is configuring conditions
  (bind _returnvalue (Actor|GetActorOfClass "/Game/FirstPerson/Blueprints/BP_FirstPersonCharacter.BP_FirstPersonCharacter_C"))
  (Pawn|Components|CharacterMovement|DisableMovement (Variables|/Script/Engine.Character|GetCharacterMovement _returnvalue))
  ;[0.15 0.15 0.15 0.5] Initialising variables
  (bind _returnvalue_2 (Actor|GetActorOfClass "/Game/Modes/HUD/HUD_TrainingMode.HUD_TrainingMode_C"))
  (Variables|Default|SetHUDRef _returnvalue_2)
  (bind _returnvalue_3 (Actor|GetActorOfClass "/Game/Actors/TrainingMode/BP_TrainingVesselSpawner.BP_TrainingVesselSpawner_C"))
  (Variables|Default|SetTestSpawnerRef _returnvalue_3)
  (bind _returnvalue_4 (Actor|GetActorOfClass "/Game/Actors/TrainingMode/BP_TrainingModeShip.BP_TrainingModeShip_C"))
  (bind _output_get (Variables|Default|SetTrainingMenuVesselRef _returnvalue_4))
  (Utilities|IsValid _output_get
    (:Is%20Valid
      (Variables|Default|SetTrainingMenuVesselRef _output_get))
    (:Is%20Not%20Valid
      (CallFunction|SpawnDisplayVessel)))
  ;[0.15 0.15 0.15 0.5] Binding functionality to HUD_TrainingMode Event Dispatchers: Start Test, End Test
  (bind _trainingmenuref (Default|GetTrainingMenu (Variables|Default|GetHUDRef)))
  (EventDispatchers|BindEventtoStartTest _trainingmenuref (delegate Custom|StartTest))
  (bind _traininguiref (Default|GetTrainingUI (Variables|Default|GetHUDRef)))
  (EventDispatchers|BindEventtoEndTest _traininguiref (delegate Custom|EndEvent)))

(fn ConstructionScript)

(fn SpawnDisplayVessel
  (bind _returnvalue (Game|SpawnActorfromClass "/Game/Actors/TrainingMode/BP_TrainingModeShip.BP_TrainingModeShip_C" (Variables|Default|GetTrainingMenuVesselTransform) "Undefined" "MultiplyWithRoot" 0 0))
  (Variables|Default|SetTrainingMenuVesselRef _returnvalue))