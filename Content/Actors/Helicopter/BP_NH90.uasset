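; BP_NH90 is a grabbable NH90 helicopter actor that works with the VR freeplay vessel controller.
; On BeginPlay it finds and caches the BP_VRFreeplayVesselController in the level.
; When the GrabComponent is dropped, the Body's physics simulation follows that controller's PhysicsEnabled setting.
; Tick spins the Blades by a fixed yaw step each frame, so rotor speed depends on frame rate.
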(event OnDropped(GrabComponent)
  (Physics|SetSimulatePhysics (Variables|Default|GetBody) (Variables|/Game/Actors/Freeplay/BP_VRFreeplayVesselController.BP_VRFreeplayVesselController_C|GetPhysicsEnabled (Variables|Default|GetControllerRef))))

(event EventBeginPlay
  (bind _returnvalue (Actor|GetActorOfClass "/Game/Actors/Freeplay/BP_VRFreeplayVesselController.BP_VRFreeplayVesselController_C"))
  (Utilities|IsValid _returnvalue
    (:Is%20Valid
      (Variables|Default|SetControllerRef _returnvalue))))

(event EventTick
  (params (DeltaSeconds :type Float%20%28single-precision%29))
  (Transformation|AddRelativeRotation (Variables|Default|GetBlades) "0.000000,20.000000,0.000000" false false))

(fn ConstructionScript)