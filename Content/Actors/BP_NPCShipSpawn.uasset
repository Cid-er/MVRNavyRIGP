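; Spawner actor that populates its SpawnArea box with random NPC ship traffic and one random threat on BeginPlay.
; Each spawn gets a random XY point and yaw, and is pushed away from existing traffic that lies within SpawnBuffer.
; A helicopter threat skips that spacing and spawns at a random high altitude, while other threats get a fixed downward offset.
; The spawned threat is passed to BP_Periscope.
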(event EventBeginPlay
  (CallFunction|NPCSpawner)
  (CallFunction|EnemySpawner))

(fn ConstructionScript)

(fn NPCSpawner
  (Variables|Default|SetShipsToSpawn (Math|Random|RandomIntegerinRange 0 3))
  (for _index (range 0 (- (Variables|Default|GetShipsToSpawn) 1))
    (CallFunction|SetNewSpawnPosition)
    (CallFunction|SetNewSpawnRotation)
    (if (== (Utilities|Array|Length (Variables|Default|GetSpawnedTraffic)) 0)
      _
      (else
        (for _index_2 (range 0 (- (Utilities|Array|Length (Variables|Default|GetSpawnedTraffic)) 1))
          (if (> (Math|Vector|Distance(Vector) (Transformation|GetActorLocation (Utilities|Array|Get(acopy) (Variables|Default|GetSpawnedTraffic) _index_2)) (Variables|Default|GetSpawnPoint)) (Variables|Default|GetSpawnBuffer))
            (Development|PrintString "good")
            (else
              (Variables|Default|SetSpawnPoint (+ (Variables|Default|GetSpawnPoint) (* (Class|KismetMathLibrary|VectorNormal2D (- (Variables|Default|GetSpawnPoint) (Transformation|GetActorLocation (Utilities|Array|Get(acopy) (Variables|Default|GetSpawnedTraffic) _index_2))) 0.0001) (Variables|Default|GetSpawnBuffer))))
              (Math|Integer|DecrementInt _index_2))))))
    (bind _returnvalue (Game|SpawnActorfromClass (Variables|Default|GetTrafficClass) (Math|Transform|MakeTransform (Variables|Default|GetSpawnPoint) (Variables|Default|GetSpawnRotation)) "Undefined" "MultiplyWithRoot" 0 0))
    (Utilities|Array|Add (Variables|Default|GetSpawnedTraffic) _returnvalue)))

(fn EnemySpawner
  (Variables|Default|SetThreatToSpawn (Math|Random|RandomInteger (Utilities|Array|Length (Variables|Default|GetThreatClass))))
  (CallFunction|SetNewSpawnPosition)
  (CallFunction|SetNewSpawnRotation)
  (if (== (Utilities|Array|Get(acopy) (Variables|Default|GetThreatClass) (Variables|Default|GetThreatToSpawn)) "/Game/Actors/NPCTraffic/BP_ThreatHelicopter.BP_ThreatHelicopter_C")
    (Variables|Default|SetThreatHeight (Math|Random|RandomFloatinRange 1.2e+04 2e+04))
    (else
      (Variables|Default|SetThreatHeight -4e+02)
      (for _index (range 0 (- (Utilities|Array|Length (Variables|Default|GetSpawnedTraffic)) 1))
        (if (> (Math|Vector|Distance(Vector) (Transformation|GetActorLocation (Utilities|Array|Get(acopy) (Variables|Default|GetSpawnedTraffic) _index)) (Variables|Default|GetSpawnPoint)) (Variables|Default|GetSpawnBuffer))
          (Development|PrintString "good")
          (else
            (Variables|Default|SetSpawnPoint (+ (Variables|Default|GetSpawnPoint) (* (Class|KismetMathLibrary|VectorNormal2D (- (Variables|Default|GetSpawnPoint) (Transformation|GetActorLocation (Utilities|Array|Get(acopy) (Variables|Default|GetSpawnedTraffic) _index))) 0.0001) (Variables|Default|GetSpawnBuffer))))
            (Math|Integer|DecrementInt _index))))))
  (bind _returnvalue (Game|SpawnActorfromClass (Utilities|Array|Get(acopy) (Variables|Default|GetThreatClass) (Variables|Default|GetThreatToSpawn)) (Math|Transform|MakeTransform (+ (Variables|Default|GetSpawnPoint) (Math|Vector|MakeVector 0.0 0.0 (Variables|Default|GetThreatHeight))) (Variables|Default|GetSpawnRotation)) "Undefined" "MultiplyWithRoot" 0 0))
  (bind _output_get (Variables|Default|SetThreat _returnvalue))
  (bind _returnvalue_2 (Actor|GetActorOfClass "/Game/Actors/BP_Periscope.BP_Periscope_C"))
  (Default|SetThreat _returnvalue_2 _output_get))

(fn SetNewSpawnPosition
  (bind _spawnarea (Variables|Default|GetSpawnArea))
  (bind _spawnarea_2 (Variables|Default|GetSpawnArea))
  (bind _returnvalue (Components|Box|GetScaledBoxExtent _spawnarea_2))
  (bind _returnvalue_2 (Transformation|GetWorldLocation _spawnarea))
  (bind _returnvalue_3 (Math|Random|RandomPointinBoundingBox _returnvalue_2 _returnvalue))
  (bind (_x _y) (Math|Vector|BreakVector _returnvalue_3))
  (Variables|Default|SetSpawnPoint (Math|Vector|MakeVector _x _y (Variables|Default|GetSpawnHeight))))

(fn SetNewSpawnRotation
  (Variables|Default|SetSpawnRotation (Math|Rotator|MakeRotator 0.0 0.0 (Math|Random|RandomFloatinRange 0.0 3.6e+02))))