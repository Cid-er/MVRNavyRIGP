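; VR periscope actor with two grabbable grips that steer a camera.
; While both grips are held, Tick yaws the rotation point from the horizontal line between the grip boxes and shows the pawn's widget.
; Rolling a box past a threshold from its reference cube adjusts clamped camera height (left) or pitch (right).
; Released boxes snap back to their cubes; stepped scene-capture zoom logic exists but is unwired.
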(event OnComponentBeginOverlap(Box)
  (params (OverlappedComponent :type Primitive%20Component%20Object%20Reference) (OtherActor :type Actor%20Object%20Reference) (OtherComp :type Primitive%20Component%20Object%20Reference) (OtherBodyIndex :type Integer) (bFromSweep :type Boolean) (SweepResult :type Hit%20Result%20Structure%20%28by%20ref%29))
  (bind _returnvalue (Game|Player|GetPlayerPawn 0))
  (bind _returnvalue_2 (Actor|GetComponentbyClass _returnvalue "/Script/UMG.WidgetComponent"))
  (if true
    (Rendering|SetVisibility _returnvalue_2 true false)
    (else
      (Rendering|SetVisibility _returnvalue_2 false false))))

(event OnDropped(Grip_R)
  (bind _cube_r (Variables|Default|GetCube_R))
  (Transformation|SetWorldLocationAndRotation (Variables|Default|GetBox_R) (Transformation|GetWorldLocation _cube_r) (Transformation|GetWorldRotation _cube_r) false true)
  (Variables|Default|SetIsRGrabbed false))

(event OnDropped(Grip_L)
  (bind _cube_l (Variables|Default|GetCube_L))
  (Transformation|SetWorldLocationAndRotation (Variables|Default|GetBox_L) (Transformation|GetWorldLocation _cube_l) (Transformation|GetWorldRotation _cube_l) false true)
  (Variables|Default|SetIsLGrabbed false))

(event OnGrabbed(Grip_L)
  (Variables|Default|SetIsLGrabbed true))

(event OnGrabbed(Grip_R)
  (Variables|Default|SetIsRGrabbed true))

(event EventTick
  (params (DeltaSeconds :type Float%20%28single-precision%29))
  (bind _returnvalue (Game|Player|GetPlayerPawn 0))
  (bind _returnvalue_2 (Actor|GetComponentbyClass _returnvalue "/Script/UMG.WidgetComponent"))
  (Utilities|FlowControl|Sequence
    (:then_0
      (if (and (Variables|Default|GetIsLGrabbed) (Variables|Default|GetIsRGrabbed))
        (Rendering|SetVisibility _returnvalue_2 true false)
        (Transformation|SetWorldRotation (Variables|Default|GetRotationPoint) (Math|Rotator|MakeRotfromX (* (Math|Vector|NegateVector (- (Transformation|GetWorldLocation (Variables|Default|GetBox_L)) (Transformation|GetWorldLocation (Variables|Default|GetBox_R)))) "1.000000,1.000000,0.000000")) false false)
        (else
          (Rendering|SetVisibility _returnvalue_2 false false))))
    (:then_1
      (CallFunction|HeightChange))
    (:then_2
      (CallFunction|PitchChange))))

(fn ConstructionScript)

(fn GetHandReferences
  (bind _returnvalue (Game|Player|GetPlayerPawn 0))
  (bind _returnvalue_2 (Actor|GetComponentsByClass _returnvalue "/Script/HeadMountedDisplay.MotionControllerComponent"))
  (if (> (Utilities|Array|Length _returnvalue_2) 0)
    (bind _output_get (Variables|Default|SetLocalMotionControllers _returnvalue_2))
    (for (_array_element _array_index) _output_get
      (if (== _array_index 0)
        (Variables|Default|SetMC_Left _array_element)
        (else
          (Variables|Default|SetMC_Right _array_element))))
    (Development|PrintString "Done!")
    (else
      (Development|PrintString "None to detect!"))))

(fn HeightChange
  (bind _camera (Variables|Default|GetCamera))
  (bind _camera_2 (Variables|Default|GetCamera))
  (bind _relativelocation (Variables|/Script/Engine.SceneComponent|GetRelativeLocation _camera_2))
  (bind _relativelocation_2 (Variables|/Script/Engine.SceneComponent|GetRelativeLocation _camera))
  (bind (_x _y) (Math|Vector|BreakVector _relativelocation_2))
  (bind (_x_2 _y_2) (Math|Vector|BreakVector _relativelocation))
  (Utilities|FlowControl|Sequence
    (:then_0
      (if (> (.roll (Transformation|GetWorldRotation (Variables|Default|GetBox_L))) (+ (.roll (Transformation|GetWorldRotation (Variables|Default|GetCube_L))) 3e+01))
        (Variables|Default|SetPeriscopeHeight (Math|Float|Clamp(Float) (+ (Variables|Default|GetPeriscopeHeight) (* (* 1.0 (Variables|Default|GetHeightSpeed)) (Utilities|Time|GetWorldDeltaSeconds))) (Variables|Default|GetMinHeight) (Variables|Default|GetMaxHeight)))
        (Transformation|SetRelativeLocation (Variables|Default|GetCamera) (Math|Vector|MakeVector _x_2 _y_2 (Variables|Default|GetPeriscopeHeight)) false false)))
    (:then_1
      (if (< (.roll (Transformation|GetWorldRotation (Variables|Default|GetBox_L))) (- (.roll (Transformation|GetWorldRotation (Variables|Default|GetCube_L))) 3e+01))
        (Variables|Default|SetPeriscopeHeight (Math|Float|Clamp(Float) (+ (Variables|Default|GetPeriscopeHeight) (* (* -1.0 (Variables|Default|GetHeightSpeed)) (Utilities|Time|GetWorldDeltaSeconds))) (Variables|Default|GetMinHeight) (Variables|Default|GetMaxHeight)))
        (Transformation|SetRelativeLocation (Variables|Default|GetCamera) (Math|Vector|MakeVector _x _y (Variables|Default|GetPeriscopeHeight)) false false)))))

(fn PitchChange
  (Utilities|FlowControl|Sequence
    (:then_0
      (if (> (.roll (Transformation|GetWorldRotation (Variables|Default|GetBox_R))) (+ (.roll (Transformation|GetWorldRotation (Variables|Default|GetCube_R))) 3e+01))
        (Transformation|AddRelativeRotation (Variables|Default|GetCamera) (Math|Rotator|MakeRotator 0.0 (* (* 1.0 (Variables|Default|GetRotateSpeed)) (Utilities|Time|GetWorldDeltaSeconds)) 0.0) false false)))
    (:then_1
      (if (< (.roll (Transformation|GetWorldRotation (Variables|Default|GetBox_R))) (- (.roll (Transformation|GetWorldRotation (Variables|Default|GetCube_R))) 3e+01))
        (Transformation|AddRelativeRotation (Variables|Default|GetCamera) (Math|Rotator|MakeRotator 0.0 (* (* -1.0 (Variables|Default|GetRotateSpeed)) (Utilities|Time|GetWorldDeltaSeconds)) 0.0) false false)))))