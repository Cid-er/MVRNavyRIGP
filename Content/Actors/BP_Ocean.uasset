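; BP_Ocean is the ocean actor that shows an underwater post-process effect while the player is in a periscope.
; The construction script builds dynamic volume, line and blurred-line materials, sets their WaterHeight from the actor's Z and assigns them as post-process blendables.
; BeginPlay finds a desktop periscope, falling back to the VR one, and binds its enter/exit events to switch the blend weight on and off.
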(event Custom|Enable%20UnderwaterPP
  ;[0.0583 0.15 0.05273 0.5] Enables Underwater Post Process when in Periscope
  (CallFunction|TogglePostProcess true))

(event Custom|Disable%20UnderwaterPP
  ;[0.15 0.03608 0.03085 0.5] Disables Underwater Post Process when out of Periscope
  (CallFunction|TogglePostProcess false))

(event EventBeginPlay
  (Variables|/Script/Engine.PostProcessComponent|SetBlendWeight (Variables|Default|GetPostProcess) 0.0)
  ;[0.15 0.15 0.15 0.5] Checks what periscope is in the level (Desktop or VR)
  (bind _returnvalue (Actor|GetActorOfClass "/Game/Actors/BP_Periscope.BP_Periscope_C"))
  (Utilities|IsValid _returnvalue
    (:Is%20Valid
      (bind _output_get (Variables|Default|SetPeriscope _returnvalue))
      (EventDispatchers|BindEventtoEnterPeriscope _output_get (delegate Custom|Enable%20UnderwaterPP))
      (EventDispatchers|BindEventtoExitPeriscope _output_get (delegate Custom|Disable%20UnderwaterPP)))
    (:Is%20Not%20Valid
      (bind _returnvalue_2 (Actor|GetActorOfClass "/Game/Actors/BP_VRDynamicAnchoredActor.BP_VRDynamicAnchoredActor_C"))
      (Utilities|IsValid _returnvalue_2
        (:Is%20Valid
          (bind _output_get_2 (Variables|Default|SetVRPeriscope _returnvalue_2))
          (EventDispatchers|BindEventtoEnterPeriscope _output_get_2 (delegate Custom|Enable%20UnderwaterPP))
          (EventDispatchers|BindEventtoExitPeriscope _output_get_2 (delegate Custom|Disable%20UnderwaterPP)))))))

(fn ConstructionScript
  (bind _returnvalue (Transformation|GetActorLocation))
  (Utilities|FlowControl|Sequence
    (:then_0
      (bind _returnvalue_2 (Rendering|Material|CreateDynamicMaterialInstance "/Game/OceanWater/WaterLine/MaterialInstance/M_PPVolume_Inst.M_PPVolume_Inst" "None" "None" :!class /Script/Engine.KismetMaterialLibrary))
      (Variables|Default|SetPPVolume _returnvalue_2)
      (bind _returnvalue_3 (Rendering|Material|CreateDynamicMaterialInstance "/Game/OceanWater/WaterLine/MaterialInstance/M_PPLine_Inst.M_PPLine_Inst" "None" "None" :!class /Script/Engine.KismetMaterialLibrary))
      (Variables|Default|SetPPLine _returnvalue_3)
      (bind _returnvalue_4 (Rendering|Material|CreateDynamicMaterialInstance "/Game/OceanWater/WaterLine/MaterialInstance/M_PPLineBlur_Inst.M_PPLineBlur_Inst" "None" "None" :!class /Script/Engine.KismetMaterialLibrary))
      (Variables|Default|SetPPLineBlur _returnvalue_4))
    (:then_1
      (Rendering|Material|SetScalarParameterValue (Variables|Default|GetPPVolume) "WaterHeight" (.z _returnvalue) :!class /Script/Engine.MaterialInstanceDynamic)
      (Rendering|Material|SetScalarParameterValue (Variables|Default|GetPPLine) "WaterHeight" (.z _returnvalue) :!class /Script/Engine.MaterialInstanceDynamic)
      (Rendering|Material|SetScalarParameterValue (Variables|Default|GetPPLineBlur) "WaterHeight" (.z _returnvalue) :!class /Script/Engine.MaterialInstanceDynamic))
    (:then_2
      (Utilities|Struct|SetmembersinPostProcessSettings (Variables|/Script/Engine.PostProcessComponent|GetSettings (Variables|Default|GetPostProcess)) (Utilities|Struct|MakeWeightedBlendables (Utilities|Array|MakeArray (Utilities|Struct|MakeWeightedBlendable 1.0 (Variables|Default|GetPPLineBlur)) (Utilities|Struct|MakeWeightedBlendable 1.0 (Variables|Default|GetPPLine)) (Utilities|Struct|MakeWeightedBlendable 1.0 (Variables|Default|GetPPVolume))))))))

(fn TogglePostProcess
  (params (Bool :type Boolean))
  (bind _postprocess (Variables|Default|GetPostProcess))
  (if Bool
    (Variables|/Script/Engine.PostProcessComponent|SetBlendWeight _postprocess 1.0)
    (else
      (Variables|/Script/Engine.PostProcessComponent|SetBlendWeight _postprocess 0.0))))