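; Interactable table actor that opens and closes the assessment quiz widget through HUD_AssessmentMode.
; On BeginPlay it finds the HUD actor and enables input for the first player controller.
; Overlap events track whether an actor is in range, with debug prints.
; The IA_Interact input toggles the widget, opening it only in range but closing it from anywhere.
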(event Input|EnhancedActionEvents|EnhancedInputActionIA_Interact
  (params (ActionValue :type Boolean) (ElapsedSeconds :type Float%20%28double-precision%29) (TriggeredSeconds :type Float%20%28double-precision%29) (InputAction :type Input%20Action%20Object%20Reference :default "/Game/Input/Actions/IA_Interact.IA_Interact"))
  (if (Variables|Default|GetUsingQuizUI)
    (Default|RemoveAssessmentWidget (Variables|Default|GetHUDRef))
    (Variables|Default|SetUsingQuizUI false)
    (Development|PrintString (Utilities|String|ToString(Boolean) (Variables|Default|GetUsingQuizUI)))
    (elif (not (Variables|Default|GetUsingQuizUI))
      (if (Variables|Default|GetPlayerInRange)
        (Default|SetAssessmentWidget (Variables|Default|GetHUDRef))
        (Variables|Default|SetUsingQuizUI true)
        (Development|PrintString (Utilities|String|ToString(Boolean) (Variables|Default|GetUsingQuizUI)))))))

(event Collision|EventActorBeginOverlap
  (params (OtherActor :type Actor%20Object%20Reference))
  ;[0.15 0.15 0.15 0.5] Player Detection
  (Variables|Default|SetPlayerInRange true)
  (Development|PrintString "PlayerInRange of Table"))

(event Collision|EventActorEndOverlap
  (params (OtherActor :type Actor%20Object%20Reference))
  ;[0.15 0.15 0.15 0.5] Player Detection
  (Variables|Default|SetPlayerInRange false)
  (Development|PrintString "PlayerNotInRange of Table"))

(event EventBeginPlay
  (bind _returnvalue (Actor|GetActorOfClass "/Game/Modes/HUD/HUD_AssessmentMode.HUD_AssessmentMode_C"))
  (Variables|Default|SetHUDRef _returnvalue)
  (Input|EnableInput (Game|GetPlayerController 0)))

(fn ConstructionScript)