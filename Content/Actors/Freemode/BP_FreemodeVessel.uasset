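; BP_FreemodeVessel is an actor that represents a selectable vessel (helicopter, submarine, ship or plane) in Freemode.
; SelectVessel swaps its static mesh, and SetDefaultDistance sets Distance by vessel type, with shorter values for aircraft than for sea vessels.
; AddDistance returns Distance plus an offset without storing it.
; Event handlers are empty, and a location update based on Distance is left unconnected, so the actor never moves itself.
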(event EventBeginPlay)

(event Collision|EventActorBeginOverlap
  (params (OtherActor :type Actor%20Object%20Reference)))

(event EventTick
  (params (DeltaSeconds :type Float%20%28single-precision%29)))

(fn ConstructionScript)

(fn SelectVessel
  (params (VesselMesh :type Static%20Mesh%20Object%20Reference))
  (Components|StaticMesh|SetStaticMesh (Variables|Default|GetStaticMesh) VesselMesh))

(fn AddDistance
  (params (DistToAdd :type Float%20%28double-precision%29))
  (return (+ DistToAdd (Variables|Default|Getdistance))))

(fn SetDefaultDistance
  (params (NewParam :type Enum_ThreatType%20Enum :default "NewEnumerator0"))
  (switch Utilities|FlowControl|Switch|SwitchonEnum_ThreatType NewParam
    (:NewEnumerator0
      (Variables|Default|Setdistance 1.5e+03))
    (:NewEnumerator1
      (Variables|Default|Setdistance 8e+03))
    (:NewEnumerator2
      (Variables|Default|Setdistance 8e+03))
    (:NewEnumerator3
      (Variables|Default|Setdistance 1.5e+03))))