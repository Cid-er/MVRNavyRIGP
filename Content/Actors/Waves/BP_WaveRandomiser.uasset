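; BP_WaveRandomiser switches the level's ocean between Light, Standard and Heavy Gerstner wave profiles through SetWaves.
; Each profile function stores wavelength, amplitude and steepness settings, then calls ApplyWaveProperties.
; That finds a WaterBodyOcean, casts to its simple Gerstner wave generator, copies the values and calls ReconfigureWaves.
; Despite the name, the random Heavy-or-Standard pick is disconnected and BeginPlay is empty; Light values are marked as needing changes.
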(event EventBeginPlay)

(fn ConstructionScript)

(fn SetLightWaves
  ;[0.15 0.15 0.15 0.5] These values need changing
  (Variables|Default|SetMinWavelength 521.0)
  (Variables|Default|SetMaxWavelength 6e+03)
  (Variables|Default|SetWavelengthFalloff 2.0)
  (Variables|Default|SetMinAmplitude 4.0)
  (Variables|Default|SetMaxAmplitude 8e+01)
  (Variables|Default|SetAmplitudeFalloff 2.0)
  (Variables|Default|SetSmallWaveSteepness 0.0)
  (Variables|Default|SetLargeWaveSteepness 0.0)
  (Variables|Default|SetSteepnessFalloff 1.0)
  (CallFunction|ApplyWaveProperties))

(fn SetStandardWaves
  (Variables|Default|SetMinWavelength 2e+03)
  (Variables|Default|SetMaxWavelength 4e+03)
  (Variables|Default|SetWavelengthFalloff 2.0)
  (Variables|Default|SetMinAmplitude 2e+01)
  (Variables|Default|SetMaxAmplitude 1.6e+02)
  (Variables|Default|SetAmplitudeFalloff 1e+01)
  (Variables|Default|SetSmallWaveSteepness 0.0)
  (Variables|Default|SetLargeWaveSteepness 0.0)
  (Variables|Default|SetSteepnessFalloff 1.0)
  (CallFunction|ApplyWaveProperties))

(fn SetHeavyWaves
  (Variables|Default|SetMinWavelength 6e+03)
  (Variables|Default|SetMaxWavelength 8.5e+03)
  (Variables|Default|SetWavelengthFalloff 2.0)
  (Variables|Default|SetMinAmplitude 4.0)
  (Variables|Default|SetMaxAmplitude 2e+02)
  (Variables|Default|SetAmplitudeFalloff 1.0)
  (Variables|Default|SetSmallWaveSteepness 0.0)
  (Variables|Default|SetLargeWaveSteepness 0.0)
  (Variables|Default|SetSteepnessFalloff 1.0)
  (CallFunction|ApplyWaveProperties))

(fn SetPropertyValues
  (params (Gerstner%20Water%20Waves%20Simple%20Ref :type Gerstner%20Water%20Wave%20Generator%20Simple%20Object%20Reference))
  (Variables|/Script/Water.GerstnerWaterWaveGeneratorSimple|SetMinWavelength Gerstner%20Water%20Waves%20Simple%20Ref (Variables|Default|GetMinWavelength))
  (Variables|/Script/Water.GerstnerWaterWaveGeneratorSimple|SetMaxWavelength Gerstner%20Water%20Waves%20Simple%20Ref (Variables|Default|GetMaxWavelength))
  (Variables|/Script/Water.GerstnerWaterWaveGeneratorSimple|SetWavelengthFalloff Gerstner%20Water%20Waves%20Simple%20Ref (Variables|Default|GetWavelengthFalloff))
  (Variables|/Script/Water.GerstnerWaterWaveGeneratorSimple|SetMinAmplitude Gerstner%20Water%20Waves%20Simple%20Ref (Variables|Default|GetMinAmplitude))
  (Variables|/Script/Water.GerstnerWaterWaveGeneratorSimple|SetMaxAmplitude Gerstner%20Water%20Waves%20Simple%20Ref (Variables|Default|GetMaxAmplitude))
  (Variables|/Script/Water.GerstnerWaterWaveGeneratorSimple|SetAmplitudeFalloff Gerstner%20Water%20Waves%20Simple%20Ref (Variables|Default|GetAmplitudeFalloff))
  (Variables|/Script/Water.GerstnerWaterWaveGeneratorSimple|SetSmallWaveSteepness Gerstner%20Water%20Waves%20Simple%20Ref (Variables|Default|GetSmallWaveSteepness))
  (Variables|/Script/Water.GerstnerWaterWaveGeneratorSimple|SetLargeWaveSteepness Gerstner%20Water%20Waves%20Simple%20Ref (Variables|Default|GetLargeWaveSteepness))
  (Variables|/Script/Water.GerstnerWaterWaveGeneratorSimple|SetSteepnessFalloff Gerstner%20Water%20Waves%20Simple%20Ref (Variables|Default|GetSteepnessFalloff)))

(fn ApplyWaveProperties
  (bind (_gerstnerwavesref _gerstnerwavessimplegeneraterref) (CallFunction|CasttoWaterBody))
  (Utilities|IsValid _gerstnerwavesref
    (:Is%20Valid
      (Utilities|IsValid _gerstnerwavessimplegeneraterref
        (:Is%20Valid
          (CallFunction|SetPropertyValues _gerstnerwavessimplegeneraterref)
          (Class|WaveProperties|ReconfigureWaves _gerstnerwavesref))
        (:Is%20Not%20Valid
          (Development|PrintString "Gerstner Waves Generator Simple Ref Invalid"))))
    (:Is%20Not%20Valid
      (Development|PrintString "Gerster Waves Ref Invalid"))))

(fn CasttoWaterBody
  (bind _returnvalue (Actor|GetActorOfClass "/Script/Water.WaterBodyOcean"))
  (bind _asgerstner_water_waves (Utilities|Casting|CastToGerstnerWaterWaves (Class|WaterBodyComponent|GetWaterWaves (Variables|/Script/Water.WaterBody|GetWaterBodyComponent _returnvalue)))
    (:then
      (bind _asgerstner_water_wave_generator_simple (Utilities|Casting|CastToGerstnerWaterWaveGeneratorSimple (Variables|/Script/Water.GerstnerWaterWaves|GetGerstnerWaveGenerator _asgerstner_water_waves))
        (:then
          (return _asgerstner_water_waves _asgerstner_water_wave_generator_simple))
        (:CastFailed
          (Development|PrintString "2nd Cast Failed"))))
    (:CastFailed
      (Development|PrintString "1st Cast Failed"))))

(fn SetWaves
  (params (WaveProfile :type EWaveProfiles%20Enum :default "EWaveProfiles_MAX"))
  (switch Utilities|FlowControl|Switch|SwitchonEWaveProfiles WaveProfile
    (:NewEnumerator0
      (CallFunction|SetLightWaves))
    (:NewEnumerator1
      (CallFunction|SetStandardWaves))
    (:NewEnumerator2
      (CallFunction|SetHeavyWaves))))