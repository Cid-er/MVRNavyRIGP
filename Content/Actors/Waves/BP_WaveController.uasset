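; BP_WaveController switches the ocean between light, standard and heavy wave profiles, chosen by argument or at random.
; Each profile sets a different WindSpeed on an FX_OceanWater Niagara actor.
; Before each change it destroys any cached actor, then InitializeWaves adopts a matching level actor or spawns one at the origin.
; BeginPlay does nothing, and random selection also prints a debug label.
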(event EventBeginPlay)

(fn ConstructionScript)

(fn SetLightWaves
  (bind _waveniagaraactor (Variables|Default|GetWaveNiagaraActor))
  (Utilities|IsValid _waveniagaraactor
    (:Is%20Valid
      (Actor|DestroyActor _waveniagaraactor))
    (:Is%20Not%20Valid
      _))
  (CallFunction|InitializeWaves)
  (Niagara|SetNiagaraVariable(Float) (Variables|/Script/Niagara.NiagaraActor|GetNiagaraComponent (Variables|Default|GetWaveNiagaraActor)) "WindSpeed" 1e+01))

(fn SetStandardWaves
  (bind _waveniagaraactor (Variables|Default|GetWaveNiagaraActor))
  (Utilities|IsValid _waveniagaraactor
    (:Is%20Valid
      (Actor|DestroyActor _waveniagaraactor))
    (:Is%20Not%20Valid
      _))
  (CallFunction|InitializeWaves)
  (Niagara|SetNiagaraVariable(Float) (Variables|/Script/Niagara.NiagaraActor|GetNiagaraComponent (Variables|Default|GetWaveNiagaraActor)) "WindSpeed" 15.0))

(fn SetHeavyWaves
  (bind _waveniagaraactor (Variables|Default|GetWaveNiagaraActor))
  (Utilities|IsValid _waveniagaraactor
    (:Is%20Valid
      (Actor|DestroyActor _waveniagaraactor))
    (:Is%20Not%20Valid
      _))
  (CallFunction|InitializeWaves)
  (Niagara|SetNiagaraVariable(Float) (Variables|/Script/Niagara.NiagaraActor|GetNiagaraComponent (Variables|Default|GetWaveNiagaraActor)) "WindSpeed" 2e+01))

(fn SetWaves
  (params (WaveProfile :type EWaveProfiles%20Enum :default "NewEnumerator0"))
  (switch Utilities|FlowControl|Switch|SwitchonEWaveProfiles WaveProfile
    (:NewEnumerator0
      (CallFunction|SetLightWaves))
    (:NewEnumerator1
      (CallFunction|SetStandardWaves))
    (:NewEnumerator2
      (CallFunction|SetHeavyWaves))))

(fn InitializeWaves
  (bind _outactors (Actor|GetAllActorsOfClass "/Script/Niagara.NiagaraActor"))
  (bind _array_element (Utilities|Array|ForEachLoopwithBreak _outactors :!label _label)
    (:LoopBody
      (if (== (AssetData|GetAsset (Variables|/Script/Niagara.NiagaraActor|GetNiagaraComponent _array_element)) "/Game/OceanWater/Effects/FX_OceanWater.FX_OceanWater")
        (Variables|Default|SetWaveNiagaraActor _array_element)
        (goto _label Break)))
    (:Completed
      (Utilities|IsValid (Variables|Default|GetWaveNiagaraActor)
        (:Is%20Not%20Valid
          (bind _returnvalue (Game|SpawnActorfromClass "/Script/Niagara.NiagaraActor" (Math|Transform|MakeTransform "0, 0, 0") "Undefined" "MultiplyWithRoot" 0 0))
          (Class|NiagaraComponent|SetAsset (Variables|/Script/Niagara.NiagaraActor|GetNiagaraComponent _returnvalue) "/Game/OceanWater/Effects/FX_OceanWater.FX_OceanWater" true)
          (Variables|Default|SetWaveNiagaraActor _returnvalue))))))

(fn RandomiseWaves
  (switch Utilities|FlowControl|Switch|SwitchonEWaveProfiles (Utilities|Enum|ByteToEnumEWaveProfiles (Math|Conversions|ToByte(Integer) (Math|Random|RandomIntegerinRange 0 2)))
    (:NewEnumerator0
      (CallFunction|SetLightWaves)
      (Development|PrintString "LW"))
    (:NewEnumerator1
      (CallFunction|SetStandardWaves)
      (Development|PrintString "SW"))
    (:NewEnumerator2
      (CallFunction|SetHeavyWaves)
      (Development|PrintString "HW"))))