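; BP_TableInteractionTraining is an interactable table that opens and closes the training test UI in training mode.
; Overlap events track whether the player is in range, and the actor enables player input on BeginPlay to receive IA_Interact.
; Interacting in range switches HUD_TrainingMode to the test widget; interacting again restores the training widget, game-only input and a hidden cursor.
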(event Input|EnhancedActionEvents|EnhancedInputActionIA_Interact
  (params (ActionValue :type Boolean) (ElapsedSeconds :type Float%20%28double-precision%29) (TriggeredSeconds :type Float%20%28double-precision%29) (InputAction :type Input%20Action%20Object%20Reference :default "/Game/Input/Actions/IA_Interact.IA_Interact"))
  (bind _returnvalue (Game|GetPlayerController 0))
  (if (Variables|Default|GetUsingQuizUI)
    (bind _returnvalue_2 (Actor|GetActorOfClass "/Game/Modes/HUD/HUD_TrainingMode.HUD_TrainingMode_C"))
    (Default|SetTrainingUIWidget _returnvalue_2)
    (Input|SetInputModeGameOnly _returnvalue false)
    (Variables|/Script/Engine.PlayerController|SetbShowMouseCursor _returnvalue false)
    (Variables|Default|SetUsingQuizUI false)
    (Development|PrintString (Utilities|String|ToString(Boolean) (Variables|Default|GetUsingQuizUI)))
    (elif (not (Variables|Default|GetUsingQuizUI))
      (if (Variables|Default|GetPlayerInRange)
        (bind _returnvalue_3 (Actor|GetActorOfClass "/Game/Modes/HUD/HUD_TrainingMode.HUD_TrainingMode_C"))
        (Default|SetTrainingTestWidget _returnvalue_3)
        (Variables|Default|SetUsingQuizUI true)
        (Development|PrintString (Utilities|String|ToString(Boolean) (Variables|Default|GetUsingQuizUI)))))))

(event Input|EnhancedActionEvents|EnhancedInputActionIA_Interact
  (params (ActionValue :type Boolean) (ElapsedSeconds :type Float%20%28double-precision%29) (TriggeredSeconds :type Float%20%28double-precision%29) (InputAction :type Input%20Action%20Object%20Reference :default "/Game/Input/Actions/IA_Interact.IA_Interact")))

(event Collision|EventActorBeginOverlap
  (params (OtherActor :type Actor%20Object%20Reference))
  ;[0.15 0.15 0.15 0.5] Player Detection
  (Variables|Default|SetPlayerInRange true)
  (Development|PrintString "PlayerInRange of Table"))

(event Collision|EventActorEndOverlap
  (params (OtherActor :type Actor%20Object%20Reference))
  ;[0.15 0.15 0.15 0.5] Player Detection
  (Variables|Default|SetPlayerInRange false)
  (Development|PrintString "PlayerNotInRange of Table"))

(event EventBeginPlay
  (Input|EnableInput (Game|GetPlayerController 0)))

(fn ConstructionScript)