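; Procedural placement actor that builds a grid of stacked shipping containers in four colours from instanced mesh components.
; The construction script clears all instances, then loops columns and rows, using a seeded random stream for each stack's height (minimum 7) and each container's colour.
; Instances spawn in world space using actor location and scale; the Rotation yaw turns column offsets and containers, while row offsets stay on world X.
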(event EventBeginPlay)

(event Collision|EventActorBeginOverlap
  (params (OtherActor :type Actor%20Object%20Reference)))

(event EventTick
  (params (DeltaSeconds :type Float%20%28single-precision%29)))

(fn ConstructionScript
  (bind _returnvalue (Transformation|GetActorLocation))
  (bind _returnvalue_2 (Transformation|GetActorScale3D))
  (bind _rotation (Variables|Default|GetRotation))
  (bind (_x _y _z) (Math|Vector|BreakVector _returnvalue))
  (bind (_x_2 _y_2 _z_2) (Math|Vector|BreakVector _returnvalue_2))
  (bind _returnvalue_3 (Math|Conversions|ToFloat(Integer) _rotation))
  (bind _returnvalue_4 (Math|Rotator|MakeRotator 0.0 0.0 _returnvalue_3))
  (Components|InstancedStaticMesh|ClearInstances (Variables|Default|GetGreenContainer))
  (Components|InstancedStaticMesh|ClearInstances (Variables|Default|GetRedContainer))
  (Components|InstancedStaticMesh|ClearInstances (Variables|Default|GetBlueContainer))
  (Components|InstancedStaticMesh|ClearInstances (Variables|Default|GetYellowContainer))
  (Variables|Default|SetRandomStream (Math|Random|MakeRandomStream (Variables|Default|GetRandomSeed)))
  (for _index (range 0 (Variables|Default|GetColumnCount))
    (for _index_2 (range 0 (- (Variables|Default|GetRowCount) 1))
      (for _index_3 (range 0 (Math|Random|RandomIntegerinRangefromStream (Variables|Default|GetRandomStream) 7 (Variables|Default|GetStackHeight)))
        (switch int (Math|Random|RandomIntegerinRangefromStream (Variables|Default|GetRandomStream) 0 3)
          (:0
            (Components|InstancedStaticMesh|AddInstance (Variables|Default|GetBlueContainer) (Math|Transform|MakeTransform (Math|Vector|MakeVector (+ _x (.X (Math|Vector|BreakVector (Math|Vector|RotateVector (Math|Vector|MakeVector (* (Math|Conversions|ToFloat(Integer) _index) (Variables|Default|GetColumnDistance)) 0.0 (Math|Conversions|ToFloat(Integer) (* _index_3 (Variables|Default|GetHeightDistance)))) _returnvalue_4))) (* _index_2 (Variables|Default|GetRowDistance))) (+ _y (.Y (Math|Vector|BreakVector (Math|Vector|RotateVector (Math|Vector|MakeVector (* (Math|Conversions|ToFloat(Integer) _index) (Variables|Default|GetColumnDistance)) 0.0 (Math|Conversions|ToFloat(Integer) (* _index_3 (Variables|Default|GetHeightDistance)))) _returnvalue_4)))) (+ _z (.Z (Math|Vector|BreakVector (Math|Vector|RotateVector (Math|Vector|MakeVector (* (Math|Conversions|ToFloat(Integer) _index) (Variables|Default|GetColumnDistance)) 0.0 (Math|Conversions|ToFloat(Integer) (* _index_3 (Variables|Default|GetHeightDistance)))) _returnvalue_4))))) _returnvalue_4 (Math|Vector|MakeVector _x_2 _y_2 _z_2)) true))
          (:1
            (Components|InstancedStaticMesh|AddInstance (Variables|Default|GetGreenContainer) (Math|Transform|MakeTransform (Math|Vector|MakeVector (+ _x (.X (Math|Vector|BreakVector (Math|Vector|RotateVector (Math|Vector|MakeVector (* (Math|Conversions|ToFloat(Integer) _index) (Variables|Default|GetColumnDistance)) 0.0 (Math|Conversions|ToFloat(Integer) (* _index_3 (Variables|Default|GetHeightDistance)))) _returnvalue_4))) (* _index_2 (Variables|Default|GetRowDistance))) (+ _y (.Y (Math|Vector|BreakVector (Math|Vector|RotateVector (Math|Vector|MakeVector (* (Math|Conversions|ToFloat(Integer) _index) (Variables|Default|GetColumnDistance)) 0.0 (Math|Conversions|ToFloat(Integer) (* _index_3 (Variables|Default|GetHeightDistance)))) _returnvalue_4)))) (+ _z (.Z (Math|Vector|BreakVector (Math|Vector|RotateVector (Math|Vector|MakeVector (* (Math|Conversions|ToFloat(Integer) _index) (Variables|Default|GetColumnDistance)) 0.0 (Math|Conversions|ToFloat(Integer) (* _index_3 (Variables|Default|GetHeightDistance)))) _returnvalue_4))))) _returnvalue_4 (Math|Vector|MakeVector _x_2 _y_2 _z_2)) true))
          (:2
            (Components|InstancedStaticMesh|AddInstance (Variables|Default|GetRedContainer) (Math|Transform|MakeTransform (Math|Vector|MakeVector (+ _x (.X (Math|Vector|BreakVector (Math|Vector|RotateVector (Math|Vector|MakeVector (* (Math|Conversions|ToFloat(Integer) _index) (Variables|Default|GetColumnDistance)) 0.0 (Math|Conversions|ToFloat(Integer) (* _index_3 (Variables|Default|GetHeightDistance)))) _returnvalue_4))) (* _index_2 (Variables|Default|GetRowDistance))) (+ _y (.Y (Math|Vector|BreakVector (Math|Vector|RotateVector (Math|Vector|MakeVector (* (Math|Conversions|ToFloat(Integer) _index) (Variables|Default|GetColumnDistance)) 0.0 (Math|Conversions|ToFloat(Integer) (* _index_3 (Variables|Default|GetHeightDistance)))) _returnvalue_4)))) (+ _z (.Z (Math|Vector|BreakVector (Math|Vector|RotateVector (Math|Vector|MakeVector (* (Math|Conversions|ToFloat(Integer) _index) (Variables|Default|GetColumnDistance)) 0.0 (Math|Conversions|ToFloat(Integer) (* _index_3 (Variables|Default|GetHeightDistance)))) _returnvalue_4))))) _returnvalue_4 (Math|Vector|MakeVector _x_2 _y_2 _z_2)) true))
          (:3
            (Components|InstancedStaticMesh|AddInstance (Variables|Default|GetYellowContainer) (Math|Transform|MakeTransform (Math|Vector|MakeVector (+ _x (.X (Math|Vector|BreakVector (Math|Vector|RotateVector (Math|Vector|MakeVector (* (Math|Conversions|ToFloat(Integer) _index) (Variables|Default|GetColumnDistance)) 0.0 (Math|Conversions|ToFloat(Integer) (* _index_3 (Variables|Default|GetHeightDistance)))) _returnvalue_4))) (* _index_2 (Variables|Default|GetRowDistance))) (+ _y (.Y (Math|Vector|BreakVector (Math|Vector|RotateVector (Math|Vector|MakeVector (* (Math|Conversions|ToFloat(Integer) _index) (Variables|Default|GetColumnDistance)) 0.0 (Math|Conversions|ToFloat(Integer) (* _index_3 (Variables|Default|GetHeightDistance)))) _returnvalue_4)))) (+ _z (.Z (Math|Vector|BreakVector (Math|Vector|RotateVector (Math|Vector|MakeVector (* (Math|Conversions|ToFloat(Integer) _index) (Variables|Default|GetColumnDistance)) 0.0 (Math|Conversions|ToFloat(Integer) (* _index_3 (Variables|Default|GetHeightDistance)))) _returnvalue_4))))) _returnvalue_4 (Math|Vector|MakeVector _x_2 _y_2 _z_2)) true)))))))