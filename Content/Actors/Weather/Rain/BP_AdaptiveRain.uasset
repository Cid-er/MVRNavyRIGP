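; BP_AdaptiveRain is a weather actor that drives a Niagara rain effect through its RainFX component.
; Every tick it pushes its RainIntensity value into the User.RainIntensity Niagara parameter, so the effect follows changes to that variable.
; EnableRain and DisableRain switch the effect on and off by setting visibility and activating or deactivating the component.
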(event EventBeginPlay)

(event Collision|EventActorBeginOverlap
  (params (OtherActor :type Actor%20Object%20Reference)))

(event EventTick
  (params (DeltaSeconds :type Float%20%28single-precision%29))
  (Niagara|SetNiagaraVariable(Float) (Variables|Default|GetRainFX) "User.RainIntensity" (Variables|Default|GetRainIntensity)))

(fn ConstructionScript)

(fn EnableRain
  (Rendering|SetVisibility (Variables|Default|GetRainFX) true false)
  (Components|Activation|Activate (Variables|Default|GetRainFX) false))

(fn DisableRain
  (Rendering|SetVisibility (Variables|Default|GetRainFX) false false)
  (Components|Activation|Deactivate (Variables|Default|GetRainFX)))