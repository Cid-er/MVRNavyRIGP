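; BP_FogController is an actor that switches a target height fog between Light, Medium and Heavy presets.
; SetFogLevel sets the fog component's density and height falloff for the chosen level, with both values rising as the fog gets heavier.
; Tick reapplies the TestFogLevel variable every frame, so changes to that variable show immediately.
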(event EventBeginPlay)

(event Collision|EventActorBeginOverlap
  (params (OtherActor :type Actor%20Object%20Reference)))

(event EventTick
  (params (DeltaSeconds :type Float%20%28single-precision%29))
  (CallFunction|SetFogLevel (Variables|Default|GetTestFogLevel)))

(fn ConstructionScript)

(fn SetFogLevel
  (params (FogLevel :type EFogLevels%20Enum :default "NewEnumerator0"))
  (bind _targetfog (Variables|Default|GetTargetFog))
  (bind _targetfog_2 (Variables|Default|GetTargetFog))
  (bind _targetfog_3 (Variables|Default|GetTargetFog))
  (bind _component (Variables|/Script/Engine.ExponentialHeightFog|GetComponent _targetfog))
  (bind _component_2 (Variables|/Script/Engine.ExponentialHeightFog|GetComponent _targetfog_2))
  (bind _component_3 (Variables|/Script/Engine.ExponentialHeightFog|GetComponent _targetfog_3))
  (switch Utilities|FlowControl|Switch|SwitchonEFogLevels FogLevel
    (:NewEnumerator0
      (Class|ExponentialHeightFogComponent|SetFogDensity _component_2 0.01)
      (Class|ExponentialHeightFogComponent|SetFogHeightFalloff _component_2 0.2))
    (:NewEnumerator1
      (Class|ExponentialHeightFogComponent|SetFogDensity _component_3 0.03)
      (Class|ExponentialHeightFogComponent|SetFogHeightFalloff _component_3 0.3))
    (:NewEnumerator2
      (Class|ExponentialHeightFogComponent|SetFogDensity _component 0.06)
      (Class|ExponentialHeightFogComponent|SetFogHeightFalloff _component 0.5))))