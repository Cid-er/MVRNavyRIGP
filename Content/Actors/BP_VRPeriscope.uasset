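; VR periscope actor with left and right grips, meant to snap the player's hands onto it while held.
; On BeginPlay it caches the pawn's motion controllers by array order, first as left; grab and drop events set per-side gripping flags.
; Per-side update functions attach the controller and a matching skeletal mesh child to the grip, or detach only that mesh.
; Nothing shown calls these updates, as Tick's sequence is empty.
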(event OnGrabbed(GrabComp_L)
  ;[0.15 0.15 0.15 0.5] Toggle left/right grip on/off
  (Variables|Default|SetIsLeftGripping true))

(event OnDropped(GrabComp_L)
  ;[0.15 0.15 0.15 0.5] Toggle left/right grip on/off
  (Variables|Default|SetIsLeftGripping false))

(event OnGrabbed(GrabComp_R)
  ;[0.15 0.15 0.15 0.5] Toggle left/right grip on/off
  (Variables|Default|SetIsRightGripping true))

(event OnDropped(GrabComp_R)
  ;[0.15 0.15 0.15 0.5] Toggle left/right grip on/off
  (Variables|Default|SetIsRightGripping false))

(event EventBeginPlay
  ;[0.15 0.15 0.15 0.5] Get References to VR Hands
  (CallFunction|GetHandReferences))

(event EventTick
  (params (DeltaSeconds :type Float%20%28single-precision%29))
  (Utilities|FlowControl|Sequence))

(fn ConstructionScript)

(fn GetHandReferences
  (bind _returnvalue (Game|Player|GetPlayerPawn 0))
  (bind _returnvalue_2 (Actor|GetComponentsByClass _returnvalue "/Script/HeadMountedDisplay.MotionControllerComponent"))
  (if (> (Utilities|Array|Length _returnvalue_2) 0)
    (bind _output_get (Variables|Default|SetLocalMotionControllers _returnvalue_2))
    (for (_array_element _array_index) _output_get
      (if (== _array_index 0)
        (Variables|Default|SetMotionControllerLeftRef _array_element)
        (else
          (Variables|Default|SetMotionControllerRightRef _array_element))))
    (else
      (Development|PrintString "None to detect!"))))

(fn UpdateComponentAttachLeft
  (bind _returnvalue (Actor|GetComponentbyClass "/Script/Engine.SkeletalMeshComponent"))
  (bind _motioncontrollerleftref (Variables|Default|GetMotionControllerLeftRef))
  (bind _children (Components|GetChildrenComponents _motioncontrollerleftref false))
  (if (Variables|Default|GetIsLeftGripping)
    (Transformation|AttachComponentToComponent _motioncontrollerleftref (Variables|Default|GetGrip_L) "None" "SnapToTarget" "SnapToTarget" "KeepWorld" true)
    (for _array_element _children
      (if (== _returnvalue _array_element)
        (Transformation|AttachComponentToComponent _array_element (Variables|Default|GetGrip_L) "None" "SnapToTarget" "SnapToTarget" "KeepWorld" true)))
    (else
      (for _array_element_2 _children
        (if (== _returnvalue _array_element_2)
          (Transformation|DetachFromComponent _array_element_2 "KeepRelative" "KeepRelative" "KeepRelative" true))))))

(fn UpdateComponentAttachRight
  (bind _returnvalue (Actor|GetComponentbyClass "/Script/Engine.SkeletalMeshComponent"))
  (bind _motioncontrollerrightref (Variables|Default|GetMotionControllerRightRef))
  (bind _children (Components|GetChildrenComponents _motioncontrollerrightref false))
  (if (Variables|Default|GetIsRightGripping)
    (Transformation|AttachComponentToComponent _motioncontrollerrightref (Variables|Default|GetGrip_R) "None" "SnapToTarget" "SnapToTarget" "KeepWorld" true)
    (for _array_element _children
      (if (== _returnvalue _array_element)
        (Transformation|AttachComponentToComponent _array_element (Variables|Default|GetGrip_R) "None" "SnapToTarget" "SnapToTarget" "KeepWorld" true)))
    (else
      (for _array_element_2 _children
        (if (== _returnvalue _array_element_2)
          (Transformation|DetachFromComponent _array_element_2 "KeepRelative" "KeepRelative" "KeepRelative" true))))))