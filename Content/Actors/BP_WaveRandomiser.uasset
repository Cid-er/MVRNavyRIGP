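; Actor that randomises the ocean's waves at BeginPlay, choosing between a heavy and a standard preset.
; It casts the level's WaterBodyOcean waves to Gerstner waves with a simple generator, printing a message if either cast fails.
; The preset fills member variables, which are copied onto the generator with a fixed wave count before ReconfigureWaves is called.
; A light preset exists but is all zeros and unused.
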(event EventBeginPlay
  (bind _returnvalue (Actor|GetActorOfClass "/Script/Water.WaterBodyOcean"))
  (bind _asgerstner_water_waves (Utilities|Casting|CastToGerstnerWaterWaves (Class|WaterBodyComponent|GetWaterWaves (Variables|/Script/Water.WaterBody|GetWaterBodyComponent _returnvalue)))
    (:then
      (bind _asgerstner_water_wave_generator_simple (Utilities|Casting|CastToGerstnerWaterWaveGeneratorSimple (Variables|/Script/Water.GerstnerWaterWaves|GetGerstnerWaveGenerator _asgerstner_water_waves))
        (:then
          (bind _output_get (Variables|Default|SetIndex (Math|Random|RandomIntegerinRange 0 1)))
          (if (== _output_get 0)
            (CallFunction|SetHeavyWaves)
            (else
              (CallFunction|SetStandardWaves)))
          (CallFunction|ApplyWaveProperties _asgerstner_water_wave_generator_simple _asgerstner_water_waves))
        (:CastFailed
          (Development|PrintString "2nd Cast Failed"))))
    (:CastFailed
      (Development|PrintString "1st Cast Failed"))))

(event Collision|EventActorBeginOverlap
  (params (OtherActor :type Actor%20Object%20Reference)))

(event EventTick
  (params (DeltaSeconds :type Float%20%28single-precision%29)))

(fn ConstructionScript)

(fn SetPropertyValues
  (params (NewParam :type Gerstner%20Water%20Wave%20Generator%20Simple%20Object%20Reference))
  (Variables|/Script/Water.GerstnerWaterWaveGeneratorSimple|SetNumWaves NewParam 20)
  (Variables|/Script/Water.GerstnerWaterWaveGeneratorSimple|SetMinWavelength NewParam (Variables|Default|GetMinWavelength))
  (Variables|/Script/Water.GerstnerWaterWaveGeneratorSimple|SetMaxWavelength NewParam (Variables|Default|GetMaxWavelength))
  (Variables|/Script/Water.GerstnerWaterWaveGeneratorSimple|SetWavelengthFalloff NewParam (Variables|Default|GetWavelengthFalloff))
  (Variables|/Script/Water.GerstnerWaterWaveGeneratorSimple|SetMinAmplitude NewParam (Variables|Default|GetMinAmplitude))
  (Variables|/Script/Water.GerstnerWaterWaveGeneratorSimple|SetMaxAmplitude NewParam (Variables|Default|GetMaxAmplitude))
  (Variables|/Script/Water.GerstnerWaterWaveGeneratorSimple|SetAmplitudeFalloff NewParam (Variables|Default|GetAmplitudeFalloff))
  (Variables|/Script/Water.GerstnerWaterWaveGeneratorSimple|SetSmallWaveSteepness NewParam (Variables|Default|GetSmallWaveSteepness))
  (Variables|/Script/Water.GerstnerWaterWaveGeneratorSimple|SetLargeWaveSteepness NewParam (Variables|Default|GetLargeWaveSteepness))
  (Variables|/Script/Water.GerstnerWaterWaveGeneratorSimple|SetSteepnessFalloff NewParam (Variables|Default|GetSteepnessFalloff)))

(fn SetLightWaves
  (Variables|Default|SetMinWavelength 0.0)
  (Variables|Default|SetMaxWavelength 0.0)
  (Variables|Default|SetWavelengthFalloff 0.0)
  (Variables|Default|SetMinAmplitude 0.0)
  (Variables|Default|SetMaxAmplitude 0.0)
  (Variables|Default|SetAmplitudeFalloff 0.0)
  (Variables|Default|SetSmallWaveSteepness 0.0)
  (Variables|Default|SetLargeWaveSteepness 0.0)
  (Variables|Default|SetSteepnessFalloff 0.0))

(fn SetStandardWaves
  (Variables|Default|SetMinWavelength 2e+03)
  (Variables|Default|SetMaxWavelength 4e+03)
  (Variables|Default|SetWavelengthFalloff 2.0)
  (Variables|Default|SetMinAmplitude 2e+01)
  (Variables|Default|SetMaxAmplitude 1.6e+02)
  (Variables|Default|SetAmplitudeFalloff 1e+01)
  (Variables|Default|SetSmallWaveSteepness 0.0)
  (Variables|Default|SetLargeWaveSteepness 0.0)
  (Variables|Default|SetSteepnessFalloff 1.0))

(fn SetHeavyWaves
  (Variables|Default|SetMinWavelength 6e+03)
  (Variables|Default|SetMaxWavelength 8.5e+03)
  (Variables|Default|SetWavelengthFalloff 2.0)
  (Variables|Default|SetMinAmplitude 4.0)
  (Variables|Default|SetMaxAmplitude 2e+02)
  (Variables|Default|SetAmplitudeFalloff 1.0)
  (Variables|Default|SetSmallWaveSteepness 0.0)
  (Variables|Default|SetLargeWaveSteepness 0.0)
  (Variables|Default|SetSteepnessFalloff 1.0))

(fn ApplyWaveProperties
  (params (GerstnerWavesSimpleRef :type Gerstner%20Water%20Wave%20Generator%20Simple%20Object%20Reference) (GerstnerWavesRef :type Gerstner%20Water%20Waves%20Object%20Reference))
  (CallFunction|SetPropertyValues GerstnerWavesSimpleRef)
  (Class|WaveProperties|ReconfigureWaves GerstnerWavesRef))