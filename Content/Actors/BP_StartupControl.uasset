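; Startup actor that randomises the level's weather, time of day and sea state on BeginPlay.
; It finds the rain, fog, day sequence and wave actors by class, then sets each to a random value, with rain only occasional.
; Only the wave randomiser lookup is validity-checked.
; Debug prints report results, though the wave print rolls again, so it can differ from the applied profile.
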(event EventBeginPlay
  (CallFunction|RandomisedRain)
  (CallFunction|RandomisedFog)
  (CallFunction|RandomisedTime)
  (CallFunction|RandomisedWaves))

(event Collision|EventActorBeginOverlap
  (params (OtherActor :type Actor%20Object%20Reference)))

(event EventTick
  (params (DeltaSeconds :type Float%20%28single-precision%29)))

(fn ConstructionScript)

(fn RandomisedRain
  (bind _returnvalue (Actor|GetActorOfClass "/Game/Actors/Weather/Rain/BP_AdaptiveRain.BP_AdaptiveRain_C"))
  (if (>= 0.125 (Math|Random|RandomFloatinRange 0.0 1.0))
    (bind _output_get (Variables|/Game/Actors/Weather/Rain/BP_AdaptiveRain.BP_AdaptiveRain_C|SetRainIntensity _returnvalue (Math|Random|RandomFloatinRange 0.1 25.0)))
    (Development|PrintString (Utilities|String|ToString(Float) _output_get))
    (else
      (Variables|/Game/Actors/Weather/Rain/BP_AdaptiveRain.BP_AdaptiveRain_C|SetRainIntensity _returnvalue 0.0))))

(fn RandomisedFog
  (bind _returnvalue (Actor|GetActorOfClass "/Game/Actors/Weather/Fog/BP_FogController.BP_FogController_C"))
  (bind _output_get (Variables|/Game/Actors/Weather/Fog/BP_FogController.BP_FogController_C|SetTestFogLevel _returnvalue (Utilities|Enum|ByteToEnumEFogLevels (Math|Conversions|ToByte(Integer) (Math|Random|RandomIntegerinRange 0 3)))))
  (Development|PrintString (Utilities|String|EnumtoString _output_get)))

(fn RandomisedTime
  (bind _returnvalue (Actor|GetActorOfClass "/Script/DaySequence.SunMoonDaySequenceActor"))
  (Class|DaySequenceActor|SetTimeOfDay _returnvalue (Math|Conversions|ToFloat(Integer) (Math|Random|RandomIntegerinRange 0 24))))

(fn RandomisedWaves
  (bind _returnvalue (Math|Random|RandomIntegerinRange 0 2))
  (bind _returnvalue_2 (Math|Conversions|ToByte(Integer) _returnvalue))
  (bind _returnvalue_3 (Utilities|Enum|ByteToEnumEWaveProfiles _returnvalue_2))
  (bind _returnvalue_4 (Actor|GetActorOfClass "/Game/Actors/Waves/BP_WaveRandomiser.BP_WaveRandomiser_C"))
  (Utilities|IsValid _returnvalue_4
    (:Is%20Valid
      (Default|SetWaves _returnvalue_4 _returnvalue_3)
      (Development|PrintString (Utilities|String|EnumtoString _returnvalue_3)))
    (:Is%20Not%20Valid
      (Development|PrintString "No Wave Randomiser in scene"))))