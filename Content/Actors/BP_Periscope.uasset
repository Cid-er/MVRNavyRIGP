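; Usable periscope actor that the player enters via interact in range or by grabbing, blending the view to its camera and adding a HUD.
; While in use, input drives height, yaw, clamped pitch and two-step zoom with motor sounds.
; Tick flags the assigned threat as spotted once it projects on screen, letting a pausable timer count down the score.
; It also opens an assessment widget and switches off night vision and thermal on exit.
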(event OnComponentBeginOverlap(InteractTrigger)
  (params (OverlappedComponent :type Primitive%20Component%20Object%20Reference) (OtherActor :type Actor%20Object%20Reference) (OtherComp :type Primitive%20Component%20Object%20Reference) (OtherBodyIndex :type Integer) (bFromSweep :type Boolean) (SweepResult :type Hit%20Result%20Structure%20%28by%20ref%29))
  ;[0.15 0.15 0.15 0.5] Player Detection
  (bind _output_get (Variables|Default|SetplayerInRange true))
  (Development|PrintString (Utilities|String|ToString(Boolean) _output_get)))

(event OnComponentEndOverlap(InteractTrigger)
  (params (OverlappedComponent :type Primitive%20Component%20Object%20Reference) (OtherActor :type Actor%20Object%20Reference) (OtherComp :type Primitive%20Component%20Object%20Reference) (OtherBodyIndex :type Integer))
  ;[0.15 0.15 0.15 0.5] Player Detection
  (bind _output_get (Variables|Default|SetplayerInRange false))
  (Development|PrintString (Utilities|String|ToString(Boolean) _output_get)))

(event OnGrabbed(GrabComponent)
  ;[0.15 0.15 0.15 0.5] Camera Change
  (Development|PrintString "Yep")
  (CallFunction|StartUsingPeriscope))

(event OnDropped(GrabComponent)
  ;[0.15 0.15 0.15 0.5] Camera Change
  (Development|PrintString "Nop")
  (CallFunction|StopUsingPeriscope))

(event Custom|StartUsingPeriscope
  (bind _returnvalue (Game|GetPlayerController 0))
  (bind _countdownhandler (Variables|Default|GetCountdownHandler))
  ;[0.15 0.15 0.15 0.5] Camera Change
  (Default|CallEnterPeriscope)
  (Variables|Default|SetpreviousView (Pawn|GetViewTarget _returnvalue))
  (Game|Player|SetViewTargetwithBlend _returnvalue self (Variables|Default|GetcameraBlend) "VTBlend_Linear" 0.0 false)
  (Input|SetIgnoreMoveInput _returnvalue true)
  (Variables|Default|SetplayerIsUsing true)
  ;;[0.15 0.15 0.15 0.5] Add Periscope  UI to camera
  (bind _returnvalue_2 (UserInterface|CreateWidget "/Game/UI/PeriscopeUI/W_PeriscopeHUD.W_PeriscopeHUD_C"))
  (bind _output_get (Variables|Default|SetHUD _returnvalue_2))
  (UserInterface|Viewport|AddtoViewport _output_get 0)
  (if (Utilities|Time|IsValidTimerHandle _countdownhandler)
    (Utilities|Time|UnpauseTimerbyHandle _countdownhandler)))

(event Custom|StopUsingPeriscope
  (bind _returnvalue (Game|GetPlayerController 0))
  (bind _countdownhandler (Variables|Default|GetCountdownHandler))
  ;[0.15 0.15 0.15 0.5] Camera Change
  (Game|Player|SetViewTargetwithBlend _returnvalue (Variables|Default|GetpreviousView) (Variables|Default|GetcameraBlend) "VTBlend_Linear" 0.0 false)
  (Input|SetIgnoreMoveInput _returnvalue false)
  (Transformation|SetActorLocation "1860.000000,1500.000000,640.000000" false false)
  (Variables|Default|SetplayerIsUsing false)
  (Viewport|RemoveAllWidgets)
  (Default|CallExitPeriscope)
  (Development|PrintString "Removed")
  (if (Utilities|Time|IsValidTimerHandle _countdownhandler)
    (Utilities|Time|PauseTimerbyHandle _countdownhandler)
    ;;[0.15 0.15 0.15 0.5] turn off night vision
    (bind _returnvalue_2 (Actor|GetActorOfClass "/Game/UI/PeriscopeUI/BP_NVG-Light.BP_NVG-Light_C"))
    (Default|ToggleNVG-Light-OFF _returnvalue_2)
    ;;[0.15 0.15 0.15 0.5] Turn off thermal
    (bind _returnvalue_3 (Actor|GetActorOfClass "/Game/Periscope/BP_ThermalPost.BP_ThermalPost_C"))
    (Rendering|SetVisibility (Variables|/Game/Periscope/BP_ThermalPost.BP_ThermalPost_C|GetPostProcess _returnvalue_3) false false)))

(event Custom|TimeCount
  (bind _timer_countdown (Variables|Default|GetTimer%20Countdown))
  (bind _returnvalue (- _timer_countdown 1))
  ;[0.15 0.15 0.15 0.5] Camera Change
  (if (Variables|Default|GetThreatSpotted)
    (bind _result (Utilities|ManipulateIntInternal _timer_countdown _returnvalue)
      (:%20%20
        (Variables|Default|SetScore (Math|Integer|Clamp(Integer) _result 0 60))
        (Development|PrintString (Utilities|String|ToString(Integer) _returnvalue))))))

(event Input|EnhancedActionEvents|EnhancedInputActionIA_Interact
  (params (ActionValue :type Boolean) (ElapsedSeconds :type Float%20%28double-precision%29) (TriggeredSeconds :type Float%20%28double-precision%29) (InputAction :type Input%20Action%20Object%20Reference :default "/Game/Input/Actions/IA_Interact.IA_Interact"))
  ;[0.15 0.15 0.15 0.5] Camera Change
  (if (and (Variables|Default|GetplayerInRange) (Variables|Default|GetplayerCanUse))
    (if (Variables|Default|GetplayerIsUsing)
      (CallFunction|StopUsingPeriscope)
      (else
        (CallFunction|StartUsingPeriscope)
        (if (Variables|Default|GetplayerIsUsing)
          (Utilities|FlowControl|DoOnce false :!label _label
            (:Completed
              (bind _returnvalue (Utilities|Time|SetTimerbyEvent (delegate Custom|TimeCount) 1.0 true false 3.0))
              (Variables|Default|SetCountdownHandler _returnvalue)
              (CallFunction|TimeCount)))
          (else
            (goto _label Reset)))))))

(event Input|EnhancedActionEvents|EnhancedInputActionIA_PeriscopeVertical
  (params (ActionValue :type Float%20%28double-precision%29) (ElapsedSeconds :type Float%20%28double-precision%29) (TriggeredSeconds :type Float%20%28double-precision%29) (InputAction :type Input%20Action%20Object%20Reference :default "/Game/VRTemplate/Input/Actions/IA_PeriscopeVertical.IA_PeriscopeVertical"))
  (bind _persicopebody (Variables|Default|GetPersicopeBody))
  (bind _relativelocation (Variables|/Script/Engine.SceneComponent|GetRelativeLocation _persicopebody))
  (bind (_x _y) (Math|Vector|BreakVector _relativelocation))
  ;[0.15 0.15 0.15 0.5] Periscope Controls
  ;;[0.15 0.15 0.15 0.5] Periscope Height Control
  (if (Variables|Default|GetplayerIsUsing)
    (Variables|Default|SetPeriscopeHeight (Math|Float|Clamp(Float) (+ (Variables|Default|GetPeriscopeHeight) (* (* ActionValue (Variables|Default|GetHeightSpeed)) (Utilities|Time|GetWorldDeltaSeconds))) (Variables|Default|GetMinHeight) (Variables|Default|GetMaxHeight)))
    (Transformation|SetRelativeLocation _persicopebody (Math|Vector|MakeVector _x _y (Variables|Default|GetPeriscopeHeight)) false false)))

(event Input|EnhancedActionEvents|EnhancedInputActionIA_Periscope_AssessmentDebug
  (params (ActionValue :type Boolean) (ElapsedSeconds :type Float%20%28double-precision%29) (TriggeredSeconds :type Float%20%28double-precision%29) (InputAction :type Input%20Action%20Object%20Reference :default "/Game/Inputs/IA_Periscope_AssessmentDebug.IA_Periscope_AssessmentDebug"))
  (bind _returnvalue (Game|GetPlayerController 0))
  ;[0.15 0.15 0.15 0.5] Periscope Controls
  ;;[0.15 0.15 0.15 0.5] Assessment Mode
  (bind _returnvalue_2 (UserInterface|CreateWidget "/Game/UI/AssessmentTest.AssessmentTest_C" _returnvalue))
  (UserInterface|Viewport|AddtoPlayerScreen _returnvalue_2)
  (Variables|/Script/Engine.PlayerController|SetbShowMouseCursor _returnvalue true)
  (Input|SetInputModeUIOnly _returnvalue _returnvalue_2 "DoNotLock" false)
  (Widget|SetFocus (Variables|/Game/UI/AssessmentTest.AssessmentTest_C|GetButton_Helicopter _returnvalue_2)))

(event Input|EnhancedActionEvents|EnhancedInputActionIA_Periscope_Zoom
  (params (ActionValue :type Float%20%28double-precision%29) (ElapsedSeconds :type Float%20%28double-precision%29) (TriggeredSeconds :type Float%20%28double-precision%29) (InputAction :type Input%20Action%20Object%20Reference :default "/Game/Inputs/IA_Periscope_Zoom.IA_Periscope_Zoom"))
  ;[0.15 0.15 0.15 0.5] Periscope Zoom
  (if (Variables|Default|GetplayerIsUsing)
    (Utilities|FlowControl|Delay 0.05)
    (Audio|PlaySound2D "/Game/Audio/Periscope/periscope_zoom.periscope_zoom" 1.0 1.0 0.0 0 0)
    (Development|PrintString "Hello")
    (if (Variables|Default|GetplayerIsUsing)
      (if (> ActionValue 0.0)
        (bind _output_get (Variables|Default|SetCurrentZoom (Math|Integer|Clamp(Integer) (+ (Variables|Default|GetCurrentZoom) 1) 0 1)))
        (else
          (Variables|Default|SetCurrentZoom (Math|Integer|Clamp(Integer) (- (Variables|Default|GetCurrentZoom) 1) 0 1))))
      (Camera|SetFieldOfView (Variables|Default|GetCamera) (Utilities|Array|Get(acopy) (Variables|Default|GetZoomFOV) _output_get))
      (Development|PrintString (Utilities|String|ToString(Integer) (Variables|Default|GetCurrentZoom))))))

(event Input|EnhancedActionEvents|EnhancedInputActionIA_PeriscopeHorizontal
  (params (ActionValue :type Float%20%28double-precision%29) (ElapsedSeconds :type Float%20%28double-precision%29) (TriggeredSeconds :type Float%20%28double-precision%29) (InputAction :type Input%20Action%20Object%20Reference :default "/Game/VRTemplate/Input/Actions/IA_PeriscopeHorizontal.IA_PeriscopeHorizontal"))
  ;[0.15 0.15 0.15 0.5] Periscope Controls
  ;;[0.15 0.15 0.15 0.5] Periscope Rotation Control
  (if (Variables|Default|GetplayerIsUsing)
    (Transformation|AddRelativeRotation (Variables|Default|GetPersicopeBody) (Math|Rotator|MakeRotator 0.0 0.0 (* (* ActionValue (Variables|Default|GetRotateSpeed)) (Utilities|Time|GetWorldDeltaSeconds))) false false)))

(event Input|EnhancedActionEvents|EnhancedInputActionIA_PeriscopePitch
  (params (ActionValue :type Float%20%28double-precision%29) (ElapsedSeconds :type Float%20%28double-precision%29) (TriggeredSeconds :type Float%20%28double-precision%29) (InputAction :type Input%20Action%20Object%20Reference :default "/Game/Inputs/IA_PeriscopePitch.IA_PeriscopePitch"))
  (bind _returnvalue (Utilities|Time|GetWorldDeltaSeconds))
  (bind _rotatespeed (Variables|Default|GetRotateSpeed))
  (bind _camera (Variables|Default|GetCamera))
  (bind _returnvalue_2 (* ActionValue _rotatespeed))
  (bind _relativerotation (Variables|/Script/Engine.SceneComponent|GetRelativeRotation _camera))
  (bind _returnvalue_3 (* _returnvalue_2 _returnvalue))
  ;[0.15 0.15 0.15 0.5] Periscope Controls
  ;;[0.15 0.15 0.15 0.5] Periscope Pitch Control
  (if (Variables|Default|GetplayerIsUsing)
    (if (not (or (and (>= (.pitch _relativerotation) 85.0) (> _returnvalue_3 0.0)) (and (< _returnvalue_3 0.0) (<= (.pitch _relativerotation) -35.0))))
      (Transformation|AddRelativeRotation (Variables|Default|GetCamera) (Math|Rotator|MakeRotator 0.0 _returnvalue_3 0.0) false false))))

(event EventTick
  (params (DeltaSeconds :type Float%20%28single-precision%29))
  (bind _returnvalue (Game|GetPlayerController 0))
  (bind _returnvalue_2 (Viewport|GetViewportSize))
  (bind _threat (Variables|Default|GetThreat))
  (bind _returnvalue_3 (Transformation|GetActorLocation _threat))
  (bind (_x _y) (Math|Vector2D|BreakVector2D _returnvalue_2))
  (bind _screenposition (Class|GameplayStatics|ProjectWorldtoScreen _returnvalue _returnvalue_3 true))
  (bind (_x_2 _y_2) (Math|Vector2D|BreakVector2D _screenposition))
  ;[0.15 0.15 0.15 0.5] Event Tick
  ;;[0.15 0.15 0.15 0.5] Threat Spotting
  (if (Utilities|IsValid _threat)
    (if (Math|Boolean|ANDBoolean (> _x_2 0.0) (> _y_2 0.0) (< _x_2 _x) (< _y_2 _y) (not (Variables|Default|GetThreatSpotted)) (Variables|Default|GetplayerIsUsing) (Variables|Default|GetplayerCanUse))
      (Development|PrintString "Spotted")
      (Variables|Default|SetThreatSpotted true)
      (Variables|Default|SetplayerCanUse true))))

(event EventBeginPlay
  (bind _returnvalue (Transformation|GetActorLocation))
  (bind _z (Math|Vector|BreakVector _returnvalue))
  ;[0.15 0.15 0.15 0.5] Camera Change
  (Input|EnableInput (Game|GetPlayerController 0))
  (Variables|Default|SetMinHeight _z)
  (Variables|Default|SetMaxHeight (+ _z (Variables|Default|GetHeightRange))))

(event Input|MouseEvents|LeftMouseButton
  (params (Key :type Key%20Structure :default "None"))
  ;[0.15 0.15 0.15 0.5] Camera Change
  (:Pressed
    (if (Variables|Default|GetThreatSpotted)
      (Utilities|FlowControl|DoOnce false
        (:Completed
          (Audio|PlaySound2D "/Game/Audio/Periscope/Bearing/MarkBearing.MarkBearing" 1.0 1.0 0.0 0 0))))))

(event Input|KeyboardEvents|D
  (params (Key :type Key%20Structure :default "None"))
  ;[0.15 0.15 0.15 0.5] Periscope Rotation/Yaw
  (:Pressed
    (if (Variables|Default|GetplayerIsUsing)
      (Utilities|IsValid (Variables|Default|GetRotationR)
        (:Is%20Valid
          _)
        (:Is%20Not%20Valid
          (bind _returnvalue (Audio|SpawnSound2D (Variables|Default|Getzoom) 1.0 1.0 0.0 0))
          (Variables|Default|SetRotationR _returnvalue)))
      (Audio|Components|Audio|FadeIn (Variables|Default|GetRotationR) 0.2 1.0 0.0 "Linear" :!class /Script/Engine.AudioComponent)))
  (:Released
    (Utilities|IsValid (Variables|Default|GetRotationR)
      (:Is%20Valid
        (Audio|Components|Audio|FadeOut (Variables|Default|GetRotationR) 0.2 0.0 "Linear" :!class /Script/Engine.AudioComponent)))))

(event Input|KeyboardEvents|A
  (params (Key :type Key%20Structure :default "None"))
  ;[0.15 0.15 0.15 0.5] Periscope Rotation/Yaw
  (:Pressed
    (if (Variables|Default|GetplayerIsUsing)
      (Utilities|IsValid (Variables|Default|GetRotationL)
        (:Is%20Valid
          _)
        (:Is%20Not%20Valid
          (bind _returnvalue (Audio|SpawnSound2D (Variables|Default|Getzoom) 1.0 1.0 0.0 0))
          (Variables|Default|SetRotationL _returnvalue)))
      (Audio|Components|Audio|FadeIn (Variables|Default|GetRotationL) 0.2 1.0 0.0 "Linear" :!class /Script/Engine.AudioComponent)))
  (:Released
    (Utilities|IsValid (Variables|Default|GetRotationL)
      (:Is%20Valid
        (Audio|Components|Audio|FadeOut (Variables|Default|GetRotationL) 0.2 0.0 "Linear" :!class /Script/Engine.AudioComponent)))))

(event Input|KeyboardEvents|R
  (params (Key :type Key%20Structure :default "None"))
  ;[0.15 0.15 0.15 0.5] Periscope Rotation/Yaw
  (:Pressed
    (if (Variables|Default|GetplayerIsUsing)
      (Utilities|IsValid (Variables|Default|GetRotationU)
        (:Is%20Valid
          _)
        (:Is%20Not%20Valid
          (bind _returnvalue (Audio|SpawnSound2D (Variables|Default|Getzoom) 1.0 1.0 0.0 0))
          (Variables|Default|SetRotationU _returnvalue)))
      (Audio|Components|Audio|FadeIn (Variables|Default|GetRotationU) 0.2 1.0 0.0 "Linear" :!class /Script/Engine.AudioComponent)))
  (:Released
    (Utilities|IsValid (Variables|Default|GetRotationU)
      (:Is%20Valid
        (Audio|Components|Audio|FadeOut (Variables|Default|GetRotationU) 0.2 0.0 "Linear" :!class /Script/Engine.AudioComponent)))))

(event Input|KeyboardEvents|F
  (params (Key :type Key%20Structure :default "None"))
  ;[0.15 0.15 0.15 0.5] Periscope Rotation/Yaw
  (:Pressed
    (if (Variables|Default|GetplayerIsUsing)
      (Utilities|IsValid (Variables|Default|GetRotationD)
        (:Is%20Valid
          (Audio|Components|Audio|FadeIn (Variables|Default|GetRotationD) 0.2 1.0 0.0 "Linear" :!class /Script/Engine.AudioComponent))
        (:Is%20Not%20Valid
          (bind _returnvalue (Audio|SpawnSound2D (Variables|Default|Getzoom) 1.0 1.0 0.0 0))
          (Variables|Default|SetRotationD _returnvalue)))))
  (:Released
    (Utilities|IsValid (Variables|Default|GetRotationD)
      (:Is%20Valid
        (Audio|Components|Audio|FadeOut (Variables|Default|GetRotationD) 0.2 0.0 "Linear" :!class /Script/Engine.AudioComponent)))))

(event Input|KeyboardEvents|W
  (params (Key :type Key%20Structure :default "None"))
  ;[0.15 0.15 0.15 0.5] Periscope Rotation/Yaw
  (:Pressed
    (if (Variables|Default|GetplayerIsUsing)
      (Utilities|IsValid (Variables|Default|GetElevateU)
        (:Is%20Valid
          (Audio|Components|Audio|FadeIn (Variables|Default|GetElevateU) 0.2 1.0 0.0 "Linear" :!class /Script/Engine.AudioComponent))
        (:Is%20Not%20Valid
          (bind _returnvalue (Audio|SpawnSound2D (Variables|Default|GetElevation) 1.0 1.0 0.0 0))
          (Variables|Default|SetElevateU _returnvalue)))))
  (:Released
    (Utilities|IsValid (Variables|Default|GetElevateU)
      (:Is%20Valid
        (Audio|Components|Audio|FadeOut (Variables|Default|GetElevateU) 0.2 0.0 "Linear" :!class /Script/Engine.AudioComponent)))))

(event Input|KeyboardEvents|S
  (params (Key :type Key%20Structure :default "None"))
  ;[0.15 0.15 0.15 0.5] Periscope Rotation/Yaw
  (:Pressed
    (if (Variables|Default|GetplayerIsUsing)
      (Utilities|IsValid (Variables|Default|GetElevateD)
        (:Is%20Valid
          (Audio|Components|Audio|FadeIn (Variables|Default|GetElevateD) 0.2 1.0 0.0 "Linear" :!class /Script/Engine.AudioComponent))
        (:Is%20Not%20Valid
          (bind _returnvalue (Audio|SpawnSound2D (Variables|Default|GetElevation) 1.0 1.0 0.0 0))
          (Variables|Default|SetElevateD _returnvalue)))))
  (:Released
    (Utilities|IsValid (Variables|Default|GetElevateD)
      (:Is%20Valid
        (Audio|Components|Audio|FadeOut (Variables|Default|GetElevateD) 0.2 0.0 "Linear" :!class /Script/Engine.AudioComponent)))))

(fn ConstructionScript)

(fn SetThreat
  (params (Threat :type Actor%20Object%20Reference))
  (Variables|Default|SetThreat Threat))

(fn CreateAssessment
  (bind _returnvalue (Game|GetPlayerController 0))
  (Viewport|RemoveAllWidgets)
  (bind _returnvalue_2 (UserInterface|CreateWidget "/Game/UI/AssessmentTest.AssessmentTest_C" _returnvalue))
  (UserInterface|Viewport|AddtoViewport _returnvalue_2 0)
  (Variables|/Script/Engine.PlayerController|SetbShowMouseCursor _returnvalue true))