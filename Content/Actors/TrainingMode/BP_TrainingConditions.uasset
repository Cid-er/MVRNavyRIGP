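; BP_TrainingConditions is a training mode actor that exposes setters for environmental conditions: waves, rain, time of day and fog.
; Each setter finds its level actor by class (wave randomiser, adaptive rain, sun/moon day sequence or fog controller) and applies the value, clamping rain and time.
; The setters also print debug strings.
; The event graph is inactive and SetTrainingTestWidget is an empty stub.
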(event EventBeginPlay)

(event Collision|EventActorBeginOverlap
  (params (OtherActor :type Actor%20Object%20Reference)))

(event EventTick
  (params (DeltaSeconds :type Float%20%28single-precision%29)))

(fn ConstructionScript)

(fn SetWaveConditions
  (params (WaveProfile :type EWaveProfiles%20Enum :default "NewEnumerator0"))
  (bind _returnvalue (Actor|GetActorOfClass "/Game/Actors/Waves/BP_WaveRandomiser.BP_WaveRandomiser_C"))
  (Default|SetWaves _returnvalue WaveProfile)
  (Development|PrintString (Utilities|String|EnumtoString WaveProfile)))

(fn SetRainConditions
  (params (Intensity :type Float%20%28double-precision%29))
  (bind _returnvalue (Actor|GetActorOfClass "/Game/Actors/Weather/Rain/BP_AdaptiveRain.BP_AdaptiveRain_C"))
  (bind _output_get (Variables|/Game/Actors/Weather/Rain/BP_AdaptiveRain.BP_AdaptiveRain_C|SetRainIntensity _returnvalue (Math|Float|Clamp(Float) Intensity 0.0 25.0)))
  (Development|PrintString "Hello" true true "(R=0.000000,G=0.660000,B=1.000000,A=1.000000)" _output_get))

(fn SetTimeOfDay
  (params (Time :type Float%20%28double-precision%29))
  (bind _returnvalue (Math|Float|Clamp(Float) Time 0.0 24.0))
  (bind _returnvalue_2 (Actor|GetActorOfClass "/Script/DaySequence.SunMoonDaySequenceActor"))
  (Class|DaySequenceActor|SetTimeOfDay _returnvalue_2 _returnvalue)
  (Development|PrintString (Class|KismetStringLibrary|TimeSecondstoString _returnvalue)))

(fn SetFogConditions
  (params (FogLevel :type EFogLevels%20Enum :default "NewEnumerator3"))
  (bind _returnvalue (Actor|GetActorOfClass "/Game/Actors/Weather/Fog/BP_FogController.BP_FogController_C"))
  (Variables|/Game/Actors/Weather/Fog/BP_FogController.BP_FogController_C|SetTestFogLevel _returnvalue FogLevel)
  (Development|PrintString (Utilities|String|EnumtoString FogLevel)))

(fn SetTrainingTestWidget)