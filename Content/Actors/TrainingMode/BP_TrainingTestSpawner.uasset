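; Training-mode spawner actor that creates a test vessel of a requested threat type (helicopter, submarine, ship or plane) around the periscope.
; SpawnTestVessel filters the threat data table by type, spawns a random matching actor class and returns it.
; SetSpawnLocation picks a random angle and distance around BP_Periscope, then adds a per-type height.
; Debug prints remain, and the printed class name re-rolls the random index, so it can differ from the spawned class.
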(fn ConstructionScript)

(fn SpawnTestVessel
  (params (ThreatType :type Enum_ThreatType%20Enum :default "NewEnumerator0"))
  (bind _spawnablevessels (Variables|Default|GetSpawnableVessels))
  (bind _returnvalue (Utilities|Array|Length _spawnablevessels))
  (bind _returnvalue_2 (- _returnvalue 1))
  (bind _returnvalue_3 (Math|Random|RandomIntegerinRange 0 _returnvalue_2))
  (bind _output (Utilities|Array|Get(acopy) _spawnablevessels _returnvalue_3))
  (Utilities|Array|Clear (Variables|Default|GetSpawnableVessels))
  (bind _outrownames (DataTable|GetDataTableRowNames "/Game/Resources/DataTableThreat.DataTableThreat"))
  (for _array_element _outrownames
    (bind _returnvalue_4 (Utilities|GetDataTableRow "/Game/Resources/DataTableThreat.DataTableThreat" _array_element)
      (:then
        (if (Utilities|Enum|Equal(Enum) (.type _returnvalue_4) ThreatType)
          (Utilities|Array|Add (Variables|Default|GetSpawnableVessels) (.bp_actorclass _returnvalue_4))))))
  (bind _location (CallFunction|SetSpawnLocation ThreatType))
  (Development|PrintString (Utilities|String|ToString(Transform) _location))
  (bind _returnvalue_5 (Game|SpawnActorfromClass _output _location "Undefined" "MultiplyWithRoot" 0 0))
  (Development|PrintString (Utilities|GetClassDisplayName _output))
  (Development|PrintString "svdvzvsdv\\")
  (return _returnvalue_5))

(fn SetSpawnLocation
  (params (ThreatType :type Enum_ThreatType%20Enum :default "NewEnumerator0"))
  (Variables|Default|SetSpawnAngle (Math|Random|RandomFloatinRange 0.0 3.6e+02))
  (Variables|Default|SetSpawnDistance (Math|Random|RandomFloatinRange (Variables|Default|GetMinSpawnDistance) (Variables|Default|GetMaxSpawnDistance)))
  (bind _returnvalue (Actor|GetActorOfClass "/Game/Actors/BP_Periscope.BP_Periscope_C"))
  (Variables|Default|SetSpawnLocation (Math|Vector|MakeVector (+ (.x (Transformation|GetActorLocation _returnvalue)) (* (Math|Trig|Cos(Degrees) (Variables|Default|GetSpawnAngle)) (Variables|Default|GetSpawnDistance))) (+ (.y (Transformation|GetActorLocation _returnvalue)) (* (Variables|Default|GetSpawnDistance) (Math|Trig|Sin(Degrees) (Variables|Default|GetSpawnAngle)))) 0.0))
  (switch Utilities|FlowControl|Switch|SwitchonEnum_ThreatType ThreatType
    (:NewEnumerator0
      (bind _output_get (Variables|Default|SetSpawnHeight 8e+03))
      (Variables|Default|SetSpawnLocation (+ (Variables|Default|GetSpawnLocation) (Math|Vector|MakeVector 0.0 0.0 _output_get))))
    (:NewEnumerator1
      (bind _output_get_2 (Variables|Default|SetSpawnHeight 0.0))
      (Variables|Default|SetSpawnLocation (+ (Variables|Default|GetSpawnLocation) (Math|Vector|MakeVector 0.0 0.0 _output_get_2))))
    (:NewEnumerator2
      (bind _output_get_3 (Variables|Default|SetSpawnHeight 2.1e+02))
      (Variables|Default|SetSpawnLocation (+ (Variables|Default|GetSpawnLocation) (Math|Vector|MakeVector 0.0 0.0 _output_get_3))))
    (:NewEnumerator3
      (bind _output_get_4 (Variables|Default|SetSpawnHeight 8e+03))
      (Variables|Default|SetSpawnLocation (+ (Variables|Default|GetSpawnLocation) (Math|Vector|MakeVector 0.0 0.0 _output_get_4)))))
  (return (Math|Transform|MakeTransform (Variables|Default|GetSpawnLocation) (Variables|Default|GetSpawnRotation) "1.000000,1.000000,1.000000")))