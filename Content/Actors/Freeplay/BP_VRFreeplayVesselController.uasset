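; BP_VRFreeplayVesselController manages the displayed vessel in VR freeplay, swapping it on request and toggling its physics.
; ChangeVessel updates the name text, destroys the current vessel and spawns the given class at the spawn point, scaled down by one of three factors chosen from the vessel type.
; EnablePhysics flips a stored flag and applies it to the vessel's static mesh, and newly spawned vessels inherit that physics state when it is on.
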(event EventBeginPlay)

(fn ConstructionScript)

(fn ChangeVessel
  (params (VesselClass :type Actor%20Class%20Reference) (VesselName :type Text) (VesselType :type Enum_ThreatType%20Enum :default "NewEnumerator0"))
  (bind _vesselspawnpoint (Variables|Default|GetVesselSpawnPoint))
  (Rendering|Components|TextRender|SetText (Variables|Default|GetTextRender) VesselName)
  (Utilities|IsValid (Variables|Default|GetVesselActor)
    (:Is%20Valid
      (Actor|DestroyActor (Variables|Default|GetVesselActor)))
    (:Is%20Not%20Valid
      _))
  (if (Utilities|Enum|Equal(Enum) VesselType "NewEnumerator5")
    (Variables|Default|SetVesselScale "0.005000,0.005000,0.005000")
    (elif (or (Utilities|Enum|Equal(Enum) VesselType "NewEnumerator0") (Utilities|Enum|Equal(Enum) VesselType "NewEnumerator3"))
      (Variables|Default|SetVesselScale "0.050000,0.050000,0.050000")
      (else
        (Variables|Default|SetVesselScale "0.010000,0.010000,0.010000"))))
  (bind _returnvalue (Game|SpawnActorfromClass VesselClass (Math|Transform|MakeTransform (Transformation|GetWorldLocation _vesselspawnpoint) (Transformation|GetWorldRotation _vesselspawnpoint) (Variables|Default|GetVesselScale)) "Undefined" "MultiplyWithRoot" 0 0))
  (Variables|Default|SetVesselActor _returnvalue)
  (if (Variables|Default|GetPhysicsEnabled)
    (Physics|SetSimulatePhysics (Actor|GetComponentbyClass (Variables|Default|GetVesselActor) "/Script/Engine.StaticMeshComponent") true)))

(fn EnablePhysics
  (bind _vesselactor (Variables|Default|GetVesselActor))
  (bind _returnvalue (Actor|GetComponentbyClass _vesselactor "/Script/Engine.StaticMeshComponent"))
  (if (Variables|Default|GetPhysicsEnabled)
    (Variables|Default|SetPhysicsEnabled false)
    (Physics|SetSimulatePhysics _returnvalue false)
    (else
      (Variables|Default|SetPhysicsEnabled true)
      (Physics|SetSimulatePhysics _returnvalue true))))