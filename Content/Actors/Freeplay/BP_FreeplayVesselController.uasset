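; Freeplay controller that spawns a selected vessel and lets the player change its distance and rotate it.
; ChangeVessel replaces the current actor, placing it on the X axis at a per-type default distance, with a larger one for the Charles de Gaulle.
; BP_FreeplayCharacter events drive scaled local rotation and distance, clamped between that default and a maximum.
; Distance adjustment omits destroyers, cargo ships and carriers, although spawning groups them with frigates.
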(event Custom|Pitch
  (params (Pitch :type Float%20%28double-precision%29))
  (bind _vesselactor (Variables|Default|GetVesselActor))
  (Utilities|IsValid _vesselactor
    (:Is%20Valid
      (Transformation|AddActorLocalRotation _vesselactor (Math|Rotator|MakeRotator 0.0 (* Pitch (Variables|Default|GetRotationSpeed)) 0.0) false false))))

(event Custom|Yaw
  (params (Yaw :type Float%20%28double-precision%29))
  (bind _vesselactor (Variables|Default|GetVesselActor))
  (bind _rotationspeed (Variables|Default|GetRotationSpeed))
  (bind _returnvalue (* Yaw _rotationspeed))
  (Utilities|IsValid _vesselactor
    (:Is%20Valid
      (Transformation|AddActorLocalRotation _vesselactor (Math|Rotator|MakeRotator 0.0 0.0 _returnvalue) false false)
      (Development|PrintString (Utilities|String|ToString(Float) _returnvalue)))))

(event Custom|Roll
  (params (Roll :type Float%20%28double-precision%29))
  (bind _rotationspeed (Variables|Default|GetRotationSpeed))
  (bind _vesselactor (Variables|Default|GetVesselActor))
  (bind _returnvalue (* Roll _rotationspeed))
  (Utilities|IsValid _vesselactor
    (:Is%20Valid
      (Transformation|AddActorLocalRotation _vesselactor (Math|Rotator|MakeRotator _returnvalue 0.0 0.0) false false)
      (Development|PrintString (Utilities|String|ToString(Float) _returnvalue)))))

(event Custom|VesselDistance
  (params (DistInput :type Float%20%28double-precision%29))
  (CallFunction|AddDistance (* DistInput (Variables|Default|GetVesselSpeed)))
  (Transformation|SetActorLocation (Variables|Default|GetVesselActor) (Math|Vector|MakeVector (Variables|Default|GetDistance) 0.0 0.0) false false))

(event EventBeginPlay
  (bind _returnvalue (Actor|GetActorOfClass "/Game/Actors/Freeplay/BP_FreeplayCharacter.BP_FreeplayCharacter_C"))
  (bind _output_get (Variables|Default|SetPlayerRef _returnvalue))
  (EventDispatchers|BindEventtoVesselDistance _output_get (delegate Custom|VesselDistance))
  (EventDispatchers|BindEventtoVesselPitch (Variables|Default|GetPlayerRef) (delegate Custom|Pitch))
  (EventDispatchers|BindEventtoVesselYaw (Variables|Default|GetPlayerRef) (delegate Custom|Yaw))
  (EventDispatchers|BindEventtoVesselRoll (Variables|Default|GetPlayerRef) (delegate Custom|Roll)))

(fn ConstructionScript)

(fn AddDistance
  (params (DistToAdd :type Float%20%28double-precision%29))
  (switch Utilities|FlowControl|Switch|SwitchonEnum_ThreatType (Variables|Default|GetVesselType)
    (:NewEnumerator0
      (Variables|Default|SetDistance (Math|Float|Clamp(Float) (+ DistToAdd (Variables|Default|GetDistance)) (Variables|Default|GetHeliDefaultDist) (Variables|Default|GetMaxDist))))
    (:NewEnumerator1
      (Variables|Default|SetDistance (Math|Float|Clamp(Float) (+ DistToAdd (Variables|Default|GetDistance)) (Variables|Default|GetSubDefaultDist) (Variables|Default|GetMaxDist))))
    (:NewEnumerator2
      (Variables|Default|SetDistance (Math|Float|Clamp(Float) (+ DistToAdd (Variables|Default|GetDistance)) (Variables|Default|GetShipDefaultDist) (Variables|Default|GetMaxDist))))
    (:NewEnumerator3
      (Variables|Default|SetDistance (Math|Float|Clamp(Float) (+ DistToAdd (Variables|Default|GetDistance)) (Variables|Default|GetPlaneDefaultDist) (Variables|Default|GetMaxDist))))))

(fn ChangeVessel
  (params (ThreatType :type Enum_ThreatType%20Enum :default "NewEnumerator0") (ThreatClass :type Actor%20Class%20Reference))
  (bind _output_get (Variables|Default|SetVesselType ThreatType))
  (switch Utilities|FlowControl|Switch|SwitchonEnum_ThreatType _output_get
    (:NewEnumerator0
      (Variables|Default|SetDistance (Variables|Default|GetHeliDefaultDist)))
    (:NewEnumerator1
      (Variables|Default|SetDistance (Variables|Default|GetSubDefaultDist)))
    (:NewEnumerator2
      (if (== "/Game/Actors/Ships/BP_CharlesDeGaulle.BP_CharlesDeGaulle_C" ThreatClass) :!label _label
        (Variables|Default|SetShipDefaultDist 1.75e+04)
        (else
          (Variables|Default|SetShipDefaultDist 1.2e+04)))
      (Variables|Default|SetDistance (Variables|Default|GetShipDefaultDist)))
    (:NewEnumerator3
      (Variables|Default|SetDistance (Variables|Default|GetPlaneDefaultDist)))
    (:NewEnumerator4
      (goto _label))
    (:NewEnumerator5
      (goto _label))
    (:NewEnumerator6
      (goto _label)))
  (Utilities|IsValid (Variables|Default|GetVesselActor)
    (:Is%20Valid
      (Actor|DestroyActor (Variables|Default|GetVesselActor)))
    (:Is%20Not%20Valid
      _))
  (bind _returnvalue (Game|SpawnActorfromClass ThreatClass (Math|Transform|MakeTransform (Math|Vector|MakeVector (Variables|Default|GetDistance) 0.0 0.0) "0, 0, 0" "1.000000,1.000000,1.000000") "Undefined" "MultiplyWithRoot" 0 0))
  (Variables|Default|SetVesselActor _returnvalue)
  (Development|PrintString (Utilities|String|ToString(Vector) (Math|Vector|MakeVector (Variables|Default|GetDistance) 0.0 0.0))))