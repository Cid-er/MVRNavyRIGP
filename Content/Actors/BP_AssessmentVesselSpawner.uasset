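; Spawner that populates a periscope assessment scene at BeginPlay with up to three random traffic vessels and one random threat from a data table.
; Each gets a random yaw and a position within a distance ring around the player, with height set by vessel type above the ocean actor.
; Spawns too close to existing traffic are nudged away by a buffer.
; The threat is passed to BP_Periscope for detection; SetNewVelocity is an unfinished stub.
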(event EventBeginPlay
  (CallFunction|SpawnTraffic)
  (CallFunction|SpawnThreat))

(fn ConstructionScript)

(fn SpawnTraffic
  ;[0.15 0.15 0.15 0.5] Randomises the NumOfTraffic to spawn
  (bind _output_get (Variables|Default|SetNumOfTraffic (Math|Random|RandomIntegerinRange 0 3)))
  (if (not (== _output_get 0))
    ;[0.15 0.15 0.15 0.5] Spawns each traffic actor via a For Loop
    (for _index (range 0 (- (Variables|Default|GetNumOfTraffic) 1))
      (CallFunction|SetNewSpawnLocation "NewEnumerator2")
      (CallFunction|SetNewSpawnRotation)
      (if (== (Utilities|Array|Length (Variables|Default|GetSpawnedTraffic)) 0)
        _
        (else
          ;[0.15 0.15 0.15 0.5] Collision prevention
          (for _index_2 (range 0 (- (Utilities|Array|Length (Variables|Default|GetSpawnedTraffic)) 1))
            (if (> (Math|Vector|Distance(Vector) (Transformation|GetActorLocation (Utilities|Array|Get(acopy) (Variables|Default|GetSpawnedTraffic) _index_2)) (Variables|Default|GetSpawnLocation)) (Variables|Default|GetSpawnBuffer))
              (Development|PrintString "good")
              (else
                (Variables|Default|SetSpawnLocation (+ (Variables|Default|GetSpawnLocation) (* (Class|KismetMathLibrary|VectorNormal2D (- (Variables|Default|GetSpawnLocation) (Transformation|GetActorLocation (Utilities|Array|Get(acopy) (Variables|Default|GetSpawnedTraffic) _index_2))) 0.0001) (Variables|Default|GetSpawnBuffer))))
                (Math|Integer|DecrementInt _index_2))))))
      (bind _returnvalue (Game|SpawnActorfromClass (Variables|Default|GetTrafficClass) (Math|Transform|MakeTransform (Variables|Default|GetSpawnLocation) (Variables|Default|GetSpawnRotation)) "Undefined" "MultiplyWithRoot" 0 0))
      (Utilities|Array|Add (Variables|Default|GetSpawnedTraffic) _returnvalue))))

(fn SpawnThreat
  ;[0.15 0.15 0.15 0.5] Randomly selects a threat to spawn from the DataTableThreat
  (bind _outrownames (DataTable|GetDataTableRowNames "/Game/Resources/DataTableThreat.DataTableThreat"))
  (bind _result (Math|Integer|DecrementInt (Utilities|Array|Length _outrownames))
    (:%20%20
      (bind _output_get (Variables|Default|SetThreatIndex (Math|Random|RandomIntegerinRange 0 _result)))
      (Development|PrintString (Utilities|String|ToString(Name) (Utilities|Array|Get(acopy) _outrownames _output_get)) true true "(R=1.000000,G=0.000000,B=0.000000,A=1.000000)" 6e+01)
      ;[0.15 0.15 0.15 0.5] Spawns the selected actor from DataTableThreat
      (bind _returnvalue (Utilities|GetDataTableRow "/Game/Resources/DataTableThreat.DataTableThreat" (Utilities|Array|Get(acopy) _outrownames _output_get))
        (:then
          (Development|PrintString (.name _returnvalue) true true "(R=1.000000,G=1.000000,B=1.000000,A=1.000000)" 6e+01)
          (CallFunction|SetNewSpawnLocation (.type _returnvalue))
          (CallFunction|SetNewSpawnRotation)
          (if (== (Variables|Default|GetNumOfTraffic) 0)
            _
            (else
              ;[0.15 0.15 0.15 0.5] Collision Prevention
              (for _index (range 0 (- (Utilities|Array|Length (Variables|Default|GetSpawnedTraffic)) 1))
                (if (> (Math|Vector|Distance(Vector) (Transformation|GetActorLocation (Utilities|Array|Get(acopy) (Variables|Default|GetSpawnedTraffic) _index)) (Variables|Default|GetSpawnLocation)) (Variables|Default|GetSpawnBuffer))
                  (Development|PrintString "Good Spawn")
                  (else
                    (Variables|Default|SetSpawnLocation (+ (Variables|Default|GetSpawnLocation) (* (Class|KismetMathLibrary|VectorNormal2D (- (Variables|Default|GetSpawnLocation) (Transformation|GetActorLocation (Utilities|Array|Get(acopy) (Variables|Default|GetSpawnedTraffic) _index))) 0.0001) (Variables|Default|GetSpawnBuffer))))
                    (Math|Integer|DecrementInt _index))))))
          (Development|PrintString (Utilities|String|ToString(Transform) (Math|Transform|MakeTransform (Variables|Default|GetSpawnLocation) (Variables|Default|GetSpawnRotation))) true true "(R=0.000000,G=0.660000,B=1.000000,A=1.000000)" 6e+01)
          (bind _returnvalue_2 (Game|SpawnActorfromClass (.bp_actorclass _returnvalue) (Math|Transform|MakeTransform (Variables|Default|GetSpawnLocation) (Variables|Default|GetSpawnRotation)) "Undefined" "MultiplyWithRoot" 0 0))
          ;[0.15 0.15 0.15 0.5] Sets the Threat in the periscope blueprint for threat detection
          (bind _output_get_2 (Variables|Default|SetThreat _returnvalue_2))
          (bind _returnvalue_3 (Actor|GetActorOfClass "/Game/Actors/BP_Periscope.BP_Periscope_C"))
          (Utilities|IsValid _returnvalue_3
            (:Is%20Valid
              (Default|SetThreat _returnvalue_3 _output_get_2))
            (:Is%20Not%20Valid
              _))
          (Default|CallSpawnedThreat))))))

(fn SetNewSpawnLocation
  (params (ThreatType :type Enum_ThreatType%20Enum :default "NewEnumerator0"))
  (bind _returnvalue (Game|Player|GetPlayerPawn 0))
  (bind _returnvalue_2 (Transformation|GetActorLocation _returnvalue))
  ;[0.15 0.15 0.15 0.5] Sets new random SpawnAngle and SpawnDistance
  (Variables|Default|SetSpawnLocation "0, 0, 0")
  (Variables|Default|SetSpawnAngle (Math|Random|RandomFloatinRange 0.0 3.6e+02))
  (Variables|Default|SetSpawnDistance (Math|Random|RandomFloatinRange (Variables|Default|GetMinSpawnDistance) (Variables|Default|GetMaxSpawnDistance)))
  ;[0.15 0.15 0.15 0.5] Multiplies the SpawnAngle by SpawnDistance to set the new SpawnLocation
  (bind _output_get (Variables|Default|SetSpawnLocation (Math|Vector|MakeVector (+ (.x _returnvalue_2) (* (Math|Trig|Cos(Degrees) (Variables|Default|GetSpawnAngle)) (Variables|Default|GetSpawnDistance))) (+ (.y _returnvalue_2) (* (Variables|Default|GetSpawnDistance) (Math|Trig|Sin(Degrees) (Variables|Default|GetSpawnAngle)))) 0.0)))
  (Development|PrintString (Utilities|String|ToString(Vector) _output_get) true true "(R=1.000000,G=0.789698,B=0.000000,A=1.000000)")
  ;[0.15 0.15 0.15 0.5] Sets the SpawnHeight based on the VesselType and height of the WaterBodyOcean in the scene
  (bind _returnvalue_3 (Actor|GetActorOfClass "/Script/Water.WaterBodyOcean"))
  (switch Utilities|FlowControl|Switch|SwitchonEnum_ThreatType ThreatType
    (:NewEnumerator0
      (bind _output_get_2 (Variables|Default|SetSpawnHeight 8e+03))
      (Variables|Default|SetSpawnLocation (+ (Variables|Default|GetSpawnLocation) (Math|Vector|MakeVector 0.0 0.0 (+ _output_get_2 (.z (Transformation|GetActorLocation _returnvalue_3)))))))
    (:NewEnumerator1
      (bind _output_get_3 (Variables|Default|SetSpawnHeight 4e+02))
      (Variables|Default|SetSpawnLocation (+ (Variables|Default|GetSpawnLocation) (Math|Vector|MakeVector 0.0 0.0 (+ _output_get_3 (.z (Transformation|GetActorLocation _returnvalue_3)))))))
    (:NewEnumerator2
      (bind _output_get_4 (Variables|Default|SetSpawnHeight 1.7e+03))
      (Variables|Default|SetSpawnLocation (+ (Variables|Default|GetSpawnLocation) (Math|Vector|MakeVector 0.0 0.0 (+ _output_get_4 (.z (Transformation|GetActorLocation _returnvalue_3)))))))
    (:NewEnumerator3
      (bind _output_get_5 (Variables|Default|SetSpawnHeight 8e+03))
      (Variables|Default|SetSpawnLocation (+ (Variables|Default|GetSpawnLocation) (Math|Vector|MakeVector 0.0 0.0 (+ _output_get_5 (.z (Transformation|GetActorLocation _returnvalue_3)))))))))

(fn SetNewSpawnRotation
  (Variables|Default|SetSpawnRotation (Math|Rotator|MakeRotator 0.0 0.0 (Math|Random|RandomFloatinRange 0.0 3.6e+02))))

(fn SetNewVelocity
  (params (Vessel :type Actor%20Object%20Reference) (VesselType :type Enum_ThreatType%20Enum :default "NewEnumerator0"))
  (switch Utilities|FlowControl|Switch|SwitchonEnum_ThreatType VesselType))